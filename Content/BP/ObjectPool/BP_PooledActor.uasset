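; BP_PooledActor is an actor meant for object pooling, switched on and off for reuse.
; It starts inactive on BeginPlay; SetInUse toggles collision, visibility and tick together to match the InUse flag.
; Activation starts a LifeSpan timer that calls ReturnToPool to deactivate the actor, and every state change clears the previous timer.
; SetInUse also takes Owner and DamageInfo, which this graph leaves unused.
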(event Custom|SetInUse
  (params (InUse :type Boolean) (Owner :type Actor%20Object%20Reference) (DamageInfo :type S%20Damage%20Info%20Structure))
  (Variables|Default|SetInUse InUse)
  (Collision|SetActorEnableCollision InUse)
  (Rendering|SetActorHiddenInGame (not InUse))
  (Actor|Tick|SetActorTickEnabled InUse)
  (Utilities|Time|ClearandInvalidateTimerbyHandle (Variables|Default|GetLifeSpanTimer))
  (if InUse
    (bind _returnvalue (Utilities|Time|SetTimerbyEvent (delegate Custom|ReturnToPool) (Variables|Default|GetLifeSpan)))
    (Variables|Default|SetLifeSpanTimer _returnvalue)))

(event Custom|ReturnToPool
  (CallFunction|SetinUse false))

(event EventBeginPlay
  (CallFunction|SetinUse false))

(fn ConstructionScript)