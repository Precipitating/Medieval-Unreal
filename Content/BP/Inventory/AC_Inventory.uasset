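; Actor component for a grid-based inventory with shaped, rotatable, stackable items, toggled on screen as a UMG widget through IA_Inventory.
; An Inventory map holds items by anchor cell, while an InventoryState map marks every cell their rotated shapes occupy.
; Pickups top up matching stacks, then try four rotations for free space, leaving any unplaced remainder on the world item.
; DropItem traces for a spawn point but ignores its item input.
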(event Input|EnhancedActionEvents|EnhancedInputActionIA_Inventory
  (params (ActionValue :type Boolean) (ElapsedSeconds :type Float%20%28double-precision%29) (TriggeredSeconds :type Float%20%28double-precision%29) (InputAction :type Input%20Action%20Object%20Reference :default "/Game/Input/Actions/IA_Inventory.IA_Inventory"))
  (bind _returnvalue (Game|GetPlayerController 0))
  (bind _returnvalue_2 (Game|GetPlayerController 0))
  (:Started
    (Variables|Default|GetUMGInventory
      (:then
        (Widget|RemovefromParent (Variables|Default|GetUMGInventory))
        (Variables|Default|SetUMGInventory 0)
        (Variables|/Script/Engine.PlayerController|SetbShowMouseCursor _returnvalue_2 false)
        (Input|SetInputModeGameOnly _returnvalue_2 false))
      (:else
        (bind _returnvalue_3 (UserInterface|CreateWidget "/Game/BP/Inventory/Widgets/UMG_Inventory.UMG_Inventory_C" 0 (Variables|Default|GetInventory) (Variables|Default|GetInventorySize) (Variables|Default|GetInventoryWidth) self))
        (bind _output_get (Variables|Default|SetUMGInventory _returnvalue_3))
        (UserInterface|Viewport|AddtoViewport _output_get 0)
        (Variables|/Script/Engine.PlayerController|SetbShowMouseCursor _returnvalue true)
        (Input|SetInputModeGameandUI _returnvalue 0 "DoNotLock" true false)))))

(event EventBeginPlay
  (State|DefaultInventoryState))

(fn DefaultInventoryState
  (for _index (range 0 (- (Variables|Default|GetInventorySize) 1))
    (Utilities|Map|Add (Variables|Default|GetInventoryState) (Math|Vector2D|MakeVector2D (LocalVariables|GetL-GridX) (LocalVariables|GetL-GridY)) false)
    (if (== (LocalVariables|GetL-GridX) (- (Variables|Default|GetInventoryWidth) 1))
      (LocalVariables|SetL-GridX 0.0)
      (Math|Float|IncrementFloat (LocalVariables|GetL-GridY))
      (else
        (Math|Float|IncrementFloat (LocalVariables|GetL-GridX)))))
  (bind _keys (Utilities|Map|Keys (Variables|Default|GetInventory)))
  (for _array_element _keys
    (State|AddtoState _array_element (.Value (Utilities|Map|Find (Variables|Default|GetInventory) _array_element)))))

(fn AddtoState
  (params (Location :type Vector%202D%20Structure) (ST_Item :type ST%20Item%20Structure%20%28by%20ref%29))
  (bind (_dataasset _rotation) (Utilities|Struct|BreakST_Item ST_Item))
  (for _array_element (Default|GetShape _dataasset _rotation)
    (Utilities|Map|Add (Variables|Default|GetInventoryState) (+ _array_element Location) true)))

(fn AddtoInventory
  (params (Key :type Vector%202D%20Structure%20%28by%20ref%29) (Value :type ST%20Item%20Structure%20%28by%20ref%29) (ModifyState :type Boolean))
  (Utilities|Map|Add (Variables|Default|GetInventory) Key Value)
  (if ModifyState
    (State|AddtoState Key Value)))

(fn RemovefromInventory
  (params (Key :type Vector%202D%20Structure) (ModifyState :type Boolean))
  (Utilities|FlowControl|Sequence
    (:then_0
      (if ModifyState
        (State|RemovefromState Key (.Value (Utilities|Map|Find (Variables|Default|GetInventory) Key)))))
    (:then_1
      (Utilities|Map|Remove (Variables|Default|GetInventory) Key))))

(fn IsNotFullyStacked
  (params (ItemStructure :type ST%20Item%20Structure))
  (bind (_dataasset _quantity) (Utilities|Struct|BreakST_Item ItemStructure))
  (bind _maxquantity (Variables|/Game/BP/Inventory_OLD/DataAssets/DA_Items.DA_Items_C|GetMaxQuantity _dataasset))
  (return (> _maxquantity _quantity) (- _maxquantity _quantity)))

(fn WhereShapeFits
  (params (Shape :type Array%20of%20Vector%202D%20Structures))
  (bind _keys (Utilities|Map|Keys (Variables|Default|GetInventoryState)))
  (for _array_element _keys
    (if (.ReturnValue (Utilities|Map|Find (Variables|Default|GetInventoryState) (- _array_element (Utilities|Array|Get(acopy) Shape))))
      (if (not (.Value (Utilities|Map|Find (Variables|Default|GetInventoryState) (- _array_element (Utilities|Array|Get(acopy) Shape)))))
        (LocalVariables|SetL-EmptySlot _array_element)
        (bind _array_element_2 (Utilities|Array|ForEachLoopwithBreak Shape :!label _label)
          (:LoopBody
            (if (or (.Value (Utilities|Map|Find (Variables|Default|GetInventoryState) (+ (LocalVariables|GetL-EmptySlot) _array_element_2))) (not (.ReturnValue (Utilities|Map|Find (Variables|Default|GetInventoryState) (+ (LocalVariables|GetL-EmptySlot) _array_element_2)))))
              (LocalVariables|SetL-Failed true)
              (goto _label Break)))
          (:Completed
            (if (LocalVariables|GetL-Failed)
              (LocalVariables|SetL-Failed false)
              (else
                (return true (LocalVariables|GetL-EmptySlot)))))))))
  (return false ""))

(fn AddItemfromFloor
  (params (ItemStructure :type ST%20Item%20Structure))
  (LocalVariables|SetL-ItemStructure ItemStructure)
  (Utilities|FlowControl|Sequence
    (:then_0
      (bind _keys (Utilities|Map|Keys (Variables|Default|GetInventory)))
      (for _array_element _keys
        (bind _output_get (LocalVariables|SetL-LoopKey _array_element))
        (LocalVariables|SetL-LoopValue (.Value (Utilities|Map|Find (Variables|Default|GetInventory) _output_get)))
        (if (== (Utilities|Struct|BreakST_Item (LocalVariables|GetL-ItemStructure)) (Utilities|Struct|BreakST_Item (LocalVariables|GetL-LoopValue)))
          (if (.ReturnValue (Conditions|IsNotFullyStacked (LocalVariables|GetL-LoopValue)))
            (Inventory|AddtoInventory (LocalVariables|GetL-LoopKey) (Utilities|Struct|MakeST_Item (.DataAsset (Utilities|Struct|BreakST_Item (LocalVariables|GetL-LoopValue))) (.Rotation (Utilities|Struct|BreakST_Item (LocalVariables|GetL-LoopValue))) (Math|Integer|Clamp(Integer) (+ (.Quantity (Utilities|Struct|BreakST_Item (LocalVariables|GetL-LoopValue))) (Utilities|Struct|BreakST_Item (LocalVariables|GetL-ItemStructure))) 0 (Variables|/Game/BP/Inventory_OLD/DataAssets/DA_Items.DA_Items_C|GetMaxQuantity (.DataAsset (Utilities|Struct|BreakST_Item (LocalVariables|GetL-LoopValue)))))) false)
            (bind _structout (Utilities|Struct|SetmembersinST_Item (LocalVariables|GetL-ItemStructure) (- (Utilities|Struct|BreakST_Item (LocalVariables|GetL-ItemStructure)) (.Remaining (Conditions|IsNotFullyStacked (LocalVariables|GetL-LoopValue))))))
            (if (<= (Utilities|Struct|BreakST_Item _structout) 0)
              (return true 0))))))
    (:then_1
      (Utilities|FlowControl|Sequence
        (:then_0
          (bind _success (Manage|CheckRotationFit (LocalVariables|GetL-ItemStructure) 0.0))
          (if _success
            (return true 0)))
        (:then_1
          (bind _success_2 (Manage|CheckRotationFit (LocalVariables|GetL-ItemStructure) 9e+01))
          (if _success_2
            (return true 0)))
        (:then_2
          (bind _success_3 (Manage|CheckRotationFit (LocalVariables|GetL-ItemStructure) 1.8e+02))
          (if _success_3
            (return true 0)))
        (:then_3
          (bind _success_4 (Manage|CheckRotationFit (LocalVariables|GetL-ItemStructure) -9e+01))
          (if _success_4
            (return true 0)))
        (:then_4
          (return false (Utilities|Struct|BreakST_Item (LocalVariables|GetL-ItemStructure))))))))

(fn DropItem
  (params (Structure :type ST%20Item%20Structure))
  (bind _returnvalue (Components|GetOwner))
  (bind _returnvalue_2 (Transformation|GetActorForwardVector _returnvalue))
  (bind _returnvalue_3 (* _returnvalue_2 2e+02))
  (bind (_outhit _returnvalue_4) (Collision|LineTraceByChannel (+ (Transformation|GetActorLocation _returnvalue) _returnvalue_3) (- _returnvalue_3 "0.000000,0.000000,500.000000") "TraceTypeQuery1" false 0 "None"))
  (if _returnvalue_4
    (Game|SpawnActorfromClass "/Game/BP/Interactables/BP_PickUpItem.BP_PickUpItem_C" (Math|Transform|MakeTransform (.ImpactPoint (Collision|BreakHitResult _outhit)) "0, 0, 0" "1.000000,1.000000,1.000000") "Undefined" "MultiplyWithRoot" 0 1.0 0 0)))

(fn PickupItem
  (params (ItemRef :type BP%20Pick%20Up%20Item%20Object%20Reference))
  (bind _remaining (Manage|AddItemfromFloor (Variables|/Game/BP/Interactables/BP_PickUpItem.BP_PickUpItem_C|GetItemStructure ItemRef)))
  (if (== _remaining 0)
    (return true)
    (else
      (Default|ModifyQuantity ItemRef _remaining)
      (return false))))

(fn RemovefromState
  (params (Location :type Vector%202D%20Structure) (ST_Item :type ST%20Item%20Structure%20%28by%20ref%29))
  (bind (_dataasset _rotation) (Utilities|Struct|BreakST_Item ST_Item))
  (for _array_element (Default|GetShape _dataasset _rotation)
    (Utilities|Map|Add (Variables|Default|GetInventoryState) (+ _array_element Location) false)))

(fn CheckRotationFit
  (params (Structure :type ST%20Item%20Structure) (Rotation :type Float%20%28double-precision%29))
  (bind _dataasset (Utilities|Struct|BreakST_Item Structure))
  (bind (_dataasset_2 _rotation _quantity) (Utilities|Struct|BreakST_Item Structure))
  (bind _defaultshape (Default|GetShape _dataasset Rotation))
  (bind (_returnvalue _validkey) (Conditions|WhereShapeFits _defaultshape))
  (if _returnvalue
    (Inventory|AddtoInventory _validkey (Utilities|Struct|MakeST_Item _dataasset_2 Rotation _quantity) true)
    (return true)
    (else
      (return false))))