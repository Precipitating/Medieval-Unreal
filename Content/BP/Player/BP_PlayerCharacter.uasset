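; Player character for a melee and crossbow combat game, handling stances, attacks, sword blocking and parrying, stat and inventory widgets, and item use.
; Input routes by stance to montages whose notifies open combo and parry windows or fire AttackComponent damage traces.
; BPC_DamageSystem handles health, blocking and attack tokens, driving hit reactions and ragdoll death.
; Weapons are cached at BeginPlay and socket-attached on equip; per-tick traces feed hand-IK wall contact.
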(event OnDamageResponse(BPC_DamageSystem)
  (params (DamageResponse :type E_DamageResponses%20Enum :default "NewEnumerator0") (DamageCauser :type Actor%20Object%20Reference) (DamageType :type E_DamageType%20Enum :default "NewEnumerator0"))
  (bind _returnvalue (Transformation|GetActorLocation))
  ;[0.15 0.15 0.15 0.5 50] ON HIT
  (Utilities|FlowControl|Sequence
    (:then_0
      ;;[0.15 0.15 0.15 0.5] Update Health Widget
      (Default|CallOnHealthUpdate)
      (Class|PlayerCharacter|SetSprint false))
    (:then_1
      (Input|DisableInput (Game|GetPlayerController 0)))
    (:then_2
      (switch Utilities|FlowControl|Switch|SwitchonE_DamageType DamageType
        (:NewEnumerator1
          (Audio|PlaySoundatLocation "/Game/Sound/Sword/PunchArmorCueHurt.PunchArmorCueHurt" _returnvalue "0, 0, 0" 1.0 1.0 0.0 0 0 0 0 :!label _label))
        (:NewEnumerator2
          (Audio|PlaySoundatLocation "/Game/Sound/Sword/SwordHitCue.SwordHitCue" _returnvalue "0, 0, 0" 1.0 1.0 0.0 0 0 0 0))
        (:NewEnumerator3
          (goto _label))
        (:NewEnumerator10
          (Audio|PlaySoundatLocation "/Game/Sound/Hurt/male_hurt7-48124.male_hurt7-48124" "0, 0, 0" "0, 0, 0" 1.0 1.0 0.0 0 0 0 0))))
    (:then_3
      (switch Utilities|FlowControl|Switch|SwitchonE_DamageResponses DamageResponse
        (:NewEnumerator0
          (Animation|Montage|PlayMontage (Variables|Character|GetMesh) "/Game/Animations/Hit/StandingReactSmallFromHeadshot_UE_Montage.StandingReactSmallFromHeadshot_UE_Montage"
            (:OnCompleted
              _)
            (:OnInterrupted
              _))
          (Input|EnableInput (Game|GetPlayerController 0)))))))

(event OnBlocked(BPC_DamageSystem)
  (params (CanBeParried :type Boolean) (DamageInfo :type E_DamageType%20Enum :default "NewEnumerator0") (DamageCauser :type Actor%20Object%20Reference))
  (bind _iswithinparrywindow (Variables|Attack|GetIsWithinParryWindow))
  (bind _returnvalue (and _iswithinparrywindow CanBeParried))
  ;[0.15 0.15 0.15 0.5 50] Block
  (Variables|Attack|SetIsReactingToBlock true)
  (switch Utilities|FlowControl|Switch|SwitchonE_DamageType DamageInfo
    (:NewEnumerator1
      (Audio|PlaySoundatLocation "/Game/Sound/Sword/PunchArmorCue.PunchArmorCue" "0, 0, 0" "0, 0, 0" 1.0 1.0 0.0 0 0 0 0))
    (:NewEnumerator2
      (switch Utilities|FlowControl|Switch|SwitchonE_PlayerStance (Variables|State|GetStance)
        (:NewEnumerator1
          (Audio|PlaySoundatLocation "/Game/Sound/Sword/SwordBlockCue.SwordBlockCue" (Transformation|GetActorLocation) "0, 0, 0" 1.0 1.0 0.0 0 0 0 0)))))
  (Animation|Montage|PlayMontage (Variables|Character|GetMesh) (select _returnvalue "/Game/Animations/Block/GreatSwordBlocking_UE_Montage.GreatSwordBlocking_UE_Montage" "/Game/Animations/Block/GreatSwordImpact_UE_Montage.GreatSwordImpact_UE_Montage")
    (:then
      (if _returnvalue
        (CallFunction|Parry DamageCauser)
        (Class|PlayerCharacter|IncreasePosture 2e+01)
        (else
          (Class|PlayerCharacter|ReducePosture (Variables|Posture|GetPostureCost)))))
    (:OnCompleted
      (CallFunction|EndBlock :!label _label))
    (:OnInterrupted
      (goto _label))))

(event OnDeath(BPC_DamageSystem)
  (params (DamageInfo :type E_DamageType%20Enum :default "NewEnumerator0"))
  (bind _mesh (Variables|Character|GetMesh))
  (bind _playerstatswidget (Variables|Widgets|Stats|GetPlayerStatsWidget))
  (bind _healthbar (Variables|/Game/UI/W_PlayerStats.W_PlayerStats_C|GetHealthBar _playerstatswidget))
  ;[0.15 0.15 0.15 0.5 50] Death
  (Audio|PlaySound2D "/Game/Sound/Death/male-death-sound-128357.male-death-sound-128357" 1.0 1.0 0.0 0 0)
  (Progress|SetPercent _healthbar 1.0)
  (Class|ProgressBar|SetFillColorandOpacity _healthbar "(R=0.000000,G=0.000000,B=0.000000,A=1.000000)")
  (Physics|SetSimulatePhysics _mesh true)
  (Collision|SetCollisionEnabled _mesh "QueryAndPhysics")
  (Input|DisableInput (Game|GetPlayerController 0)))

(event EDItemUse(InventoryComponent)
  (params (ItemObject :type BP%20Pick%20Up%20Item%20Class%20Reference))
  ;[0.15 0.15 0.15 0.5 50] Inventory
  (CallFunction|UseItem ItemObject))

(event Custom|Kick
  ;[0.15 0.15 0.15 0.5 50] KICK
  (if (not (CallFunction|IsFalling))
    (Variables|State|SetAttacking true)
    (Class|PlayerCharacter|SetKicked true)
    (bind _notifyname (Animation|Montage|PlayMontage (Variables|Character|GetMesh) "/Game/Animations/Character/Kicking_UE5_Montage.Kicking_UE5_Montage")
      (:OnCompleted
        (Class|PlayerCharacter|SetKicked false :!label _label)
        (Variables|State|SetAttacking false))
      (:OnInterrupted
        (goto _label))
      (:OnNotifyBegin
        (switch name _notifyname
          (:Kicked
            (Default|SphereTraceDamage (Variables|Default|GetAttackComponent) (Utilities|Struct|MakeS_DamageInfo 1e+01 "NewEnumerator5" "NewEnumerator1" false true false true) 2e+01 1.5e+02)))))))

(event Custom|ResetCrossbow
  (bind _camera (Variables|Default|GetCamera))
  (bind _returnvalue (Transformation|GetWorldLocation _camera))
  ;[0.15 0.15 0.15 0.5 50] Crossbow
  (Utilities|FlowControl|DoOnce false) ; enters at Reset
)

(event Custom|SwordAttack
  ;[0.15 0.15 0.15 0.5 50] Sword
  (if (not (CallFunction|IsFalling))
    (Variables|State|SetAttacking true)
    (Utilities|FlowControl|DoOnce false
      (:Completed
        (if (not (Variables|Attack|GetIsWithinComboWindow))
          (bind _notifyname (Animation|Montage|PlayMontage (Variables|Character|GetMesh) "/Game/Animations/Attacks/Sword/OneHandSwordCombo_UE_Montage.OneHandSwordCombo_UE_Montage")
            (:OnCompleted
              (Variables|State|SetAttacking false :!label _label)
              (CallFunction|SwordReset)
              (Variables|Attack|SetIsWithinComboWindow false))
            (:OnInterrupted
              (goto _label))
            (:OnNotifyBegin
              (switch name _notifyname
                (:Slashed
                  (Default|SphereTraceDamage (Variables|Default|GetAttackComponent) (Utilities|Struct|MakeS_DamageInfo 2e+01 "NewEnumerator2" "NewEnumerator0" false true true true) 2e+01 1.5e+02)
                  (Class|PlayerCharacter|ReduceStamina (Variables|Stamina|GetSwordStaminaCost)))
                (:ComboWindow
                  (Variables|Attack|SetIsWithinComboWindow true)
                  (Variables|Attack|SetCanResumeCombo false)
                  (CallFunction|SwordReset))))
            (:OnNotifyEnd
              (switch name _notifyname
                (:ComboWindow
                  (Variables|Attack|SetIsWithinComboWindow false)
                  (if (not (Variables|Attack|GetCanResumeCombo))
                    (Animation|StopAnimMontage "/Game/Animations/Attacks/Sword/OneHandSwordCombo_UE_Montage.OneHandSwordCombo_UE_Montage"))))))
          (else
            (Variables|Attack|SetCanResumeCombo true)))))))

(event Custom|PunchAttack
  ;[0.15 0.15 0.15 0.5 50] Punch
  (if (not (CallFunction|IsFalling))
    (Variables|State|SetAttacking true)
    (Utilities|FlowControl|DoOnce false
      (:Completed
        (if (not (Variables|Attack|GetIsWithinComboWindow))
          (bind _notifyname (Animation|Montage|PlayMontage (Variables|Character|GetMesh) "/Game/Animations/Attacks/Punch/PunchCombo_UE_Montage.PunchCombo_UE_Montage")
            (:OnCompleted
              (Variables|State|SetAttacking false :!label _label)
              (CallFunction|ResetPunch)
              (Variables|Attack|SetIsWithinComboWindow false))
            (:OnInterrupted
              (goto _label))
            (:OnNotifyBegin
              (switch name _notifyname
                (:Punch
                  (Default|SphereTraceDamage (Variables|Default|GetAttackComponent) (Utilities|Struct|MakeS_DamageInfo 1e+01 "NewEnumerator1" "NewEnumerator0" false true true) 2e+01 1e+02)
                  (Class|PlayerCharacter|ReduceStamina (Variables|Stamina|GetPunchStaminaCost)))
                (:ComboWindow
                  (Variables|Attack|SetIsWithinComboWindow true)
                  (Variables|Attack|SetCanResumeCombo false)
                  (CallFunction|ResetPunch))))
            (:OnNotifyEnd
              (switch name _notifyname
                (:ComboWindow
                  (Variables|Attack|SetIsWithinComboWindow false)
                  (if (not (Variables|Attack|GetCanResumeCombo))
                    (Animation|StopAnimMontage "/Game/Animations/Attacks/Punch/PunchCombo_UE_Montage.PunchCombo_UE_Montage"))))))
          (else
            (Variables|Attack|SetCanResumeCombo true)))))))

(event Custom|ResetPunch
  ;[0.15 0.15 0.15 0.5 50] Punch
  (Utilities|FlowControl|DoOnce false) ; enters at Reset
)

(event Custom|StartBlock
  ;[0.15 0.15 0.15 0.5 50] Block
  (if (Utilities|Enum|Equal(Enum) (Variables|State|GetStance) "NewEnumerator1")
    (Utilities|FlowControl|DoOnce false
      (:Completed
        (bind _notifyname (Animation|Montage|PlayMontage (Variables|Character|GetMesh) "/Game/Animations/Block/GreatSwordBlocking_UE_Montage.GreatSwordBlocking_UE_Montage")
          (:OnCompleted
            (CallFunction|EndBlock))
          (:OnInterrupted
            (if (not (Variables|Attack|GetIsReactingToBlock))
              (CallFunction|EndBlock)))
          (:OnNotifyBegin
            (switch name _notifyname
              (:Block
                (Variables|/Game/BP/Components/DamageSystemComponent.DamageSystemComponent_C|SetIsBlocking (Variables|Default|GetBPC_DamageSystem) true))
              (:ParryWindow
                (Variables|Attack|SetIsWithinParryWindow true))))
          (:OnNotifyEnd
            (switch name _notifyname
              (:ParryWindow
                (Variables|Attack|SetIsWithinParryWindow false)))))))))

(event Custom|ResetBlock
  ;[0.15 0.15 0.15 0.5 50] Block
  (Utilities|FlowControl|DoOnce false) ; enters at Reset
)

(event Custom|SwordEquip
  ;[0.15 0.15 0.15 0.5 50] Sword
  (bind _notifyname (Animation|Montage|PlayMontage (Variables|Character|GetMesh) "/Game/Animations/Attacks/Sword/UnSheathingSword_UE_Montage1.UnSheathingSword_UE_Montage1")
    (:OnNotifyBegin
      (switch name _notifyname
        (:HoldSword
          (Variables|State|SetStance "NewEnumerator1")
          (CallFunction|EquipWeapon "/Game/BP/Weapons/BP_Weapon_Sword.BP_Weapon_Sword_C" "hand_rSocket")
          (Variables|Weapons|SetIsHoldingWeapon true)
          (Default|CallOnWeaponEquip))))))

(event Custom|EndBlock
  ;[0.15 0.15 0.15 0.5 50] Block
  (Variables|/Game/BP/Components/DamageSystemComponent.DamageSystemComponent_C|SetIsBlocking (Variables|Default|GetBPC_DamageSystem) false)
  (CallFunction|ResetBlock)
  (Animation|StopAnimMontage "/Game/Animations/Block/GreatSwordBlocking_UE_Montage.GreatSwordBlocking_UE_Montage")
  (Variables|Attack|SetIsWithinParryWindow false)
  (Variables|Attack|SetIsReactingToBlock false))

(event Custom|Parry
  (params (AttackTarget :type Actor%20Object%20Reference))
  ;[0.15 0.15 0.15 0.5 50] Block
  (Class|BPIDamagable|TakeDamage(Message) AttackTarget (Utilities|Struct|MakeS_DamageInfo 5.0 "NewEnumerator6" "NewEnumerator3" false false false true) self)
  (Audio|SpawnSoundatLocation "/Game/Sound/Sword/SwordParryCue.SwordParryCue" (Transformation|GetActorLocation) "0, 0, 0" 1.0 1.0 0.0 0 0)
  (Utilities|FlowControl|Delay 0.2)
  (Utilities|Time|SetGlobalTimeDilation 0.2)
  (Utilities|FlowControl|Delay 0.1)
  (Utilities|Time|SetGlobalTimeDilation 1.0)
  (Class|PlayerCharacter|IncreaseStamina 1e+01))

(event Custom|DefaultStance
  ;[0.15 0.15 0.15 0.5 50] Punch
  (Variables|State|SetStance "NewEnumerator0")
  (CallFunction|UnEquipAllWeapons))

(event Custom|CrossbowEquip
  ;[0.15 0.15 0.15 0.5 50] Crossbow
  (Variables|State|SetStance "NewEnumerator4")
  (CallFunction|EquipWeapon "/Game/BP/Weapons/BP_Weapon_Crossbow.BP_Weapon_Crossbow_C" "hand_rSocket_crossbow")
  (Variables|Weapons|SetIsHoldingWeapon true)
  (Default|CallOnWeaponEquip))

(event Custom|OpenInventory
  (params (OtherInventory :type W%20Inventory%20Lootable%20Object%20Reference))
  ;[0.15 0.15 0.15 0.5 50] Inventory
  (if (UserInterface|Viewport|IsinViewport (Variables|Widgets|Inventory|GetInventoryWidget))
    (Widget|RemovefromParent (Variables|Widgets|Inventory|GetInventoryWidget))
    (bind _objectinventory (Variables|Widgets|Inventory|GetObjectInventory)
      (:then
        (Widget|RemovefromParent _objectinventory)
        (Variables|Widgets|Inventory|SetObjectInventory _objectinventory))
      (:else
        _))
    (Input|SetInputModeGameOnly (Game|GetPlayerController 0) false)
    (Variables|/Script/Engine.PlayerController|SetbShowMouseCursor (Game|GetPlayerController 0) false)
    (else
      (UserInterface|Viewport|AddtoViewport (Variables|Widgets|Inventory|GetInventoryWidget) 0)
      (Utilities|IsValid OtherInventory
        (:Is%20Valid
          (UserInterface|Viewport|AddtoViewport OtherInventory 0)
          (Variables|Widgets|Inventory|SetObjectInventory OtherInventory))
        (:Is%20Not%20Valid
          _))
      (Input|SetInputModeGameandUI (Game|GetPlayerController 0) 0 "DoNotLock" false false)
      (Variables|/Script/Engine.PlayerController|SetbShowMouseCursor (Game|GetPlayerController 0) true))))

(event Custom|SwordReset
  ;[0.15 0.15 0.15 0.5 50] Sword
  (Utilities|FlowControl|DoOnce false) ; enters at Reset
)

(event Custom|DisplayCrosshair
  ;[0.15 0.15 0.15 0.5 50] Crosshair
  (bind _crosshairref (Variables|Crosshair|GetCrosshairRef)
    (:then
      (Widget|SetVisibility _crosshairref "Visible"))
    (:else
      (bind _returnvalue (UserInterface|CreateWidget "/Game/UI/W_CrossHair.W_CrossHair_C"))
      (Variables|Crosshair|SetCrosshairRef _returnvalue)
      (UserInterface|Viewport|AddtoViewport _returnvalue 0))))

(event Custom|CrossbowAttack
  (bind _camera (Variables|Default|GetCamera))
  (bind _returnvalue (Transformation|GetWorldLocation _camera))
  ;[0.15 0.15 0.15 0.5 50] Crossbow
  (if (not (CallFunction|IsFalling))
    (Variables|State|SetAttacking true)
    (Utilities|FlowControl|DoOnce false
      (:Completed
        (bind _notifyname (Animation|Montage|PlayMontage (Variables|Character|GetMesh) "/Game/Animations/Attacks/Crossbow/FiringRifle_UE_Anim_Montage.FiringRifle_UE_Anim_Montage")
          (:OnCompleted
            (Default|CallOnAttackEnd :!label _label)
            (Variables|State|SetAttacking false)
            (CallFunction|ResetCrossbow))
          (:OnInterrupted
            (goto _label))
          (:OnNotifyBegin
            (switch name _notifyname
              (:Fire
                (Audio|PlaySoundatLocation "/Game/Sound/Crossbow/crossbow-firing-95020.crossbow-firing-95020" _returnvalue "0, 0, 0" 1.0 1.0 0.0 0 0 0 0)
                (Default|LineTraceDamage (Variables|Default|GetAttackComponent) (Utilities|Struct|MakeS_DamageInfo 4e+01 "NewEnumerator3" "NewEnumerator0" false false false true) _returnvalue (* (Math|Vector|GetForwardVector _camera) 6e+03) (Transformation|GetActorLocation (.Value (Utilities|Map|Find (Variables|Weapons|GetWeaponList) "/Game/BP/Weapons/BP_Weapon_Crossbow.BP_Weapon_Crossbow_C"))))
                (Class|BPIWeapon|ConsumeAmmo(Message) (.Value (Utilities|Map|Find (Variables|Weapons|GetWeaponList) "/Game/BP/Weapons/BP_Weapon_Crossbow.BP_Weapon_Crossbow_C")))))))))))

(event Input|EnhancedActionEvents|EnhancedInputActionIA_Attack
  (params (ActionValue :type Boolean) (ElapsedSeconds :type Float%20%28double-precision%29) (TriggeredSeconds :type Float%20%28double-precision%29) (InputAction :type Input%20Action%20Object%20Reference :default "/Game/Input/Actions/IA_Attack.IA_Attack"))
  (bind _weaponlist (Variables|Weapons|GetWeaponList))
  (bind _inventorycomponent (Variables|Default|GetInventoryComponent))
  (bind (_result _array_index) (Default|DoesItemExist _inventorycomponent "/Game/BP/Interactables/BP_CrossbowAmmo.BP_CrossbowAmmo_C"))
  (bind _value (Utilities|Map|Find _weaponlist "/Game/BP/Weapons/BP_Weapon_Crossbow.BP_Weapon_Crossbow_C"))
  ;[0.15 0.15 0.15 0.5 50] LMB Attacks
  (if (not (Variables|/Game/BP/Components/AttackComponent.AttackComponent_C|GetIsExecuting (Variables|Default|GetAttackComponent)))
    (switch Utilities|FlowControl|Switch|SwitchonE_PlayerStance (Variables|State|GetStance)
      (:NewEnumerator0
        (if (|(Stamina>StaminaCost) (Class|PlayerCharacter|GetStamina) (Variables|Stamina|GetPunchStaminaCost))
          (CallFunction|PunchAttack)))
      (:NewEnumerator1
        (if (|(Stamina>StaminaCost) (Class|PlayerCharacter|GetStamina) (Variables|Stamina|GetSwordStaminaCost))
          (CallFunction|SwordAttack)))
      (:NewEnumerator4
        (if (not (Variables|Weapons|GetIsReloading))
          (bind _returnvalue (Class|BPIWeapon|NeedsReload(Message) _value))
          (if _returnvalue
            (if (.Result (Default|DoesItemExist (Variables|Default|GetInventoryComponent) "/Game/BP/Interactables/BP_CrossbowAmmo.BP_CrossbowAmmo_C"))
              (Variables|Weapons|SetIsReloading true)
              (Animation|Montage|PlayMontage (Variables|Character|GetMesh) "/Game/Animations/Reload/ModernXbow_Reload_Quiver1_Montage.ModernXbow_Reload_Quiver1_Montage"
                (:OnCompleted
                  (Class|BPIWeapon|Reload(Message) _value)
                  (Variables|Weapons|SetIsReloading false)
                  (if _result
                    (Default|ReduceQuantity _inventorycomponent _array_index 1)))
                (:OnInterrupted
                  (Variables|Weapons|SetIsReloading false))))
            (else
              (CallFunction|CrossbowAttack))))))))

(event Input|EnhancedActionEvents|EnhancedInputActionIA_EquipCrossbow
  (params (ActionValue :type Boolean) (ElapsedSeconds :type Float%20%28double-precision%29) (TriggeredSeconds :type Float%20%28double-precision%29) (InputAction :type Input%20Action%20Object%20Reference :default "/Game/Input/Actions/IA_EquipCrossbow.IA_EquipCrossbow"))
  ;[0.15 0.15 0.15 0.5 50] Crossbow
  (:Started
    (if (.Result (Default|DoesItemExist (Variables|Default|GetInventoryComponent) "/Game/BP/Interactables/BP_CrossbowItem.BP_CrossbowItem_C"))
      (CallFunction|ChangeStance "NewEnumerator4"))))

(event Input|EnhancedActionEvents|EnhancedInputActionIA_Zoom
  (params (ActionValue :type Boolean) (ElapsedSeconds :type Float%20%28double-precision%29) (TriggeredSeconds :type Float%20%28double-precision%29) (InputAction :type Input%20Action%20Object%20Reference :default "/Game/Input/Actions/IA_Zoom.IA_Zoom"))
  ;[0.15 0.15 0.15 0.5 50] Zoom
  (:Triggered
    (switch Utilities|FlowControl|Switch|SwitchonE_PlayerStance (Variables|State|GetStance)
      (:NewEnumerator4
        (bind _zoomalpha (Timeline|ZoomTimeline Play)
          (:Update
            (Camera|SetFieldOfView (Variables|Default|GetCamera) (Math|Float|Lerp (Variables|FOV|GetNormalFOV) (Variables|FOV|GetZoomFOV) _zoomalpha)))))))
  (:Completed
    (Camera|SetFieldOfView (Variables|Default|GetCamera) (Variables|FOV|GetNormalFOV))
    (Utilities|String|Reverse (Variables|Default|GetZoomTimeline))))

(event Input|EnhancedActionEvents|EnhancedInputActionIA_EquipSword
  (params (ActionValue :type Boolean) (ElapsedSeconds :type Float%20%28double-precision%29) (TriggeredSeconds :type Float%20%28double-precision%29) (InputAction :type Input%20Action%20Object%20Reference :default "/Game/Input/Actions/IA_EquipSword.IA_EquipSword"))
  ;[0.15 0.15 0.15 0.5 50] Sword
  (:Started
    (if (.Result (Default|DoesItemExist (Variables|Default|GetInventoryComponent) "/Game/BP/Interactables/BP_SwordItem.BP_SwordItem_C"))
      (CallFunction|ChangeStance "NewEnumerator1"))))

(event Input|EnhancedActionEvents|EnhancedInputActionIA_Block
  (params (ActionValue :type Boolean) (ElapsedSeconds :type Float%20%28double-precision%29) (TriggeredSeconds :type Float%20%28double-precision%29) (InputAction :type Input%20Action%20Object%20Reference :default "/Game/Input/Actions/IA_Block.IA_Block"))
  (bind _stance (Variables|State|GetStance))
  ;[0.15 0.15 0.15 0.5 50] Block
  (:Triggered
    (if (not (Variables|/Game/BP/Components/AttackComponent.AttackComponent_C|GetIsExecuting (Variables|Default|GetAttackComponent)))
      (if (> (Class|PlayerCharacter|GetPosture) (Variables|Posture|GetPostureCost))
        (switch Utilities|FlowControl|Switch|SwitchonE_PlayerStance _stance
          (:NewEnumerator1
            (CallFunction|StartBlock))))))
  (:Completed
    (switch Utilities|FlowControl|Switch|SwitchonE_PlayerStance _stance
      (:NewEnumerator1
        (CallFunction|EndBlock)))))

(event Input|EnhancedActionEvents|EnhancedInputActionIA_Inventory
  (params (ActionValue :type Boolean) (ElapsedSeconds :type Float%20%28double-precision%29) (TriggeredSeconds :type Float%20%28double-precision%29) (InputAction :type Input%20Action%20Object%20Reference :default "/Game/Input/Actions/IA_Inventory.IA_Inventory"))
  ;[0.15 0.15 0.15 0.5 50] Inventory
  (:Started
    (CallFunction|OpenInventory)))

(event EventBeginPlay
  (bind _weaponlist (Variables|Weapons|GetWeaponList))
  ;[0.15 0.15 0.15 0.5 50] BEGIN PLAY
  (Utilities|FlowControl|Sequence
    (:then_0
      ;;[0.15 0.15 0.15 0.5] Stat Widget
      (bind _returnvalue (UserInterface|CreateWidget "/Game/UI/W_PlayerStats.W_PlayerStats_C" 0 self))
      (UserInterface|Viewport|AddtoViewport _returnvalue 0)
      (Variables|Widgets|Stats|SetPlayerStatsWidget _returnvalue)
      ;;[0.15 0.15 0.15 0.5] Inventory Widget
      (bind _returnvalue_2 (UserInterface|CreateWidget "/Game/BP/Inventory/Widgets/W_Inventory.W_Inventory_C" (Game|GetPlayerController 0) (Variables|Default|GetInventoryComponent) 1e+02))
      (Variables|Widgets|Inventory|SetInventoryWidget _returnvalue_2))
    (:then_1
      ;;[0.15 0.15 0.15 0.5] Crosshair
      (CallFunction|DisplayCrosshair)
      (Default|ShowCrosshair (Variables|Crosshair|GetCrosshairRef)))
    (:then_2
      (Variables|Default|SetCanMove true))
    (:then_3
      ;;[0.15 0.15 0.15 0.5] Cache weapons
      (bind _returnvalue_3 (Game|SpawnActorfromClass "/Game/BP/Weapons/BP_Weapon_Sword.BP_Weapon_Sword_C" (Math|Transform|MakeTransform "0, 0, 0" "0, 0, 0" "1.000000,1.000000,1.000000") "Undefined" "MultiplyWithRoot" 0 0))
      (Utilities|Map|Add _weaponlist "/Game/BP/Weapons/BP_Weapon_Sword.BP_Weapon_Sword_C" _returnvalue_3)
      (bind _returnvalue_4 (Game|SpawnActorfromClass "/Game/BP/Weapons/BP_Weapon_Crossbow.BP_Weapon_Crossbow_C" (Math|Transform|MakeTransform "0, 0, 0" "0, 0, 0" "1.000000,1.000000,1.000000") "Undefined" "MultiplyWithRoot" 0 0))
      (Utilities|Map|Add _weaponlist "/Game/BP/Weapons/BP_Weapon_Crossbow.BP_Weapon_Crossbow_C" _returnvalue_4))))

(event EventSetInterruptable
  (params (Interruptable :type Boolean))
  ;[0.15 0.15 0.15 0.5 50] Attack Tokens
  (Variables|/Game/BP/Components/DamageSystemComponent.DamageSystemComponent_C|SetIsInterruptible (Variables|Default|GetBPC_DamageSystem) Interruptable))

(event EventReturnAttackToken
  (params (Amount :type Integer))
  ;[0.15 0.15 0.15 0.5 50] Attack Tokens
  (Default|ReturnAttackToken (Variables|Default|GetBPC_DamageSystem) Amount))

(event EventTick
  (params (DeltaSeconds :type Float%20%28single-precision%29))
  ;[0.15 0.15 0.15 0.5 50] IK Hands
  (Utilities|FlowControl|Sequence
    (:then_0
      (bind (_hitlocation _hashitwall) (CallFunction|IKHandTrace "upperarm_lSocket" 6e+01))
      (Variables|HandsIK|SetIKLeftHandLocation _hitlocation)
      (Variables|HandsIK|SetLeftHitWall _hashitwall))
    (:then_1
      (bind (_hitlocation_2 _hashitwall_2) (CallFunction|IKHandTrace "upperarm_rSocket" 7e+01))
      (Variables|HandsIK|SetIKRightHandLocation _hitlocation_2)
      (Variables|HandsIK|SetRightHitWall _hashitwall_2))))

(fn ConstructionScript
  (Variables|/Game/BP/Components/DamageSystemComponent.DamageSystemComponent_C|SetAttackTokenCount (Variables|Default|GetBPC_DamageSystem) 2))

(fn IKHandTrace
  (params (SocketName :type Name) (Dist :type Float%20%28double-precision%29))
  (bind _returnvalue (Transformation|GetActorForwardVector))
  (bind _mesh (Variables|Character|GetMesh))
  (bind _returnvalue_2 (Transformation|GetSocketLocation _mesh SocketName))
  (bind (_outhit _returnvalue_3) (Collision|LineTraceByChannel _returnvalue_2 (+ _returnvalue_2 (* _returnvalue Dist)) "TraceTypeQuery1" false 0 "None"))
  (if _returnvalue_3
    (return (- (.location _outhit) (* _returnvalue 1e+01)) true)
    (else
      (return "0, 0, 0" false))))

(fn ChangeStance
  (params (NewStance :type E_PlayerStance%20Enum :default "NewEnumerator0"))
  (if (not (Class|AnimInstance|IsAnyMontagePlaying (Components|SkeletalMesh|GetAnimInstance (Variables|Character|GetMesh))))
    (LocalVariables|SetOldStance (Variables|State|GetStance))
    (CallFunction|DefaultStance)
    (switch Utilities|FlowControl|Switch|SwitchonE_PlayerStance NewStance
      (:NewEnumerator1
        (if (Utilities|Enum|NotEqual(Enum) (LocalVariables|GetOldStance) NewStance)
          (CallFunction|SwordEquip)))
      (:NewEnumerator4
        (if (Utilities|Enum|NotEqual(Enum) (LocalVariables|GetOldStance) NewStance)
          (CallFunction|CrossbowEquip))))))

(fn EquipWeapon
  (params (Weapon :type BP%20Weapon%20Base%20Class%20Reference) (SocketName :type Name))
  (bind _weaponlist (Variables|Weapons|GetWeaponList))
  (bind (_value _returnvalue) (Utilities|Map|Find _weaponlist Weapon))
  (if _returnvalue
    (Transformation|AttachComponentToComponent _value (Variables|Character|GetMesh) SocketName "SnapToTarget" "SnapToTarget" "SnapToTarget" true)
    (Default|SetinUse _value true)
    (return _value)
    (else
      (Development|PrintString "WEAPON NOT FOUND IN CACHE"))))

(fn UnEquipAllWeapons
  (bind _weaponlist (Variables|Weapons|GetWeaponList))
  (bind _keys (Utilities|Map|Keys _weaponlist))
  (for _array_element _keys
    (Default|SetinUse (.Value (Utilities|Map|Find _weaponlist _array_element)) false)))

(fn IsFalling
  (return (AI|Components|NavMovement|IsFalling (Variables|Character|GetCharacterMovement))))

(fn IsMontagePlaying
  (return (Class|AnimInstance|IsAnyMontagePlaying (Components|SkeletalMesh|GetAnimInstance (Variables|Character|GetMesh)))))

(fn UseItem
  (params (ItemObject :type BP%20Pick%20Up%20Item%20Class%20Reference))
  (bind _inventorycomponent (Variables|Default|GetInventoryComponent))
  (bind (_result _array_index) (Default|DoesItemExist _inventorycomponent "/Game/BP/Interactables/BP_HealthPotObject.BP_HealthPotObject_C"))
  (if (== ItemObject "/Game/BP/Interactables/BP_HealthPotObject.BP_HealthPotObject_C")
    (CallFunction|Heal (Utilities|GetClassDefaults "/Game/BP/Interactables/BP_HealthPotObject.BP_HealthPotObject_C"))
    (if _result
      (Default|ReduceQuantity _inventorycomponent _array_index 1)
      (Default|CallOnHealthUpdate))
    (elif (== ItemObject "/Game/BP/Interactables/BP_SwordItem.BP_SwordItem_C")
      (switch Utilities|FlowControl|Switch|SwitchonE_PlayerStance (Variables|State|GetStance)
        (:NewEnumerator0
          _)
        (:NewEnumerator4
          _))
      (CallFunction|ChangeStance "NewEnumerator1")
      (elif (== ItemObject "/Game/BP/Interactables/BP_CrossbowItem.BP_CrossbowItem_C")
        (switch Utilities|FlowControl|Switch|SwitchonE_PlayerStance (Variables|State|GetStance)
          (:NewEnumerator0
            _)
          (:NewEnumerator1
            _))
        (CallFunction|ChangeStance "NewEnumerator4")))))

(fn GetTraceRotation
  (bind _camera (Variables|Default|GetCamera))
  (bind _returnvalue (Transformation|GetWorldLocation _camera))
  (bind _outhit (Collision|LineTraceByChannel _returnvalue (+ _returnvalue (* (Math|Vector|GetForwardVector _camera) 1e+04)) "TraceTypeQuery1" false 0 "None" true "(R=1.000000,G=0.918511,B=0.000000,A=1.000000)" "(R=0.000000,G=1.000000,B=0.000000,A=1.000000)" 2.0))
  (return (Math|Rotator|FindLookatRotation (Transformation|GetActorLocation) (.location _outhit))))

(fn GetHealth
  (return (Variables|/Game/BP/Components/DamageSystemComponent.DamageSystemComponent_C|GetHealth (Variables|Default|GetBPC_DamageSystem))))

(fn GetMaxHealth
  (return (Variables|/Game/BP/Components/DamageSystemComponent.DamageSystemComponent_C|GetMaxHealth (Variables|Default|GetBPC_DamageSystem))))

(fn GetTeamNumber
  (return (Variables|Team|GetTeamNumber)))

(fn Heal
  (params (HealValue :type Float%20%28double-precision%29))
  (bind _newhealth (Default|Heal (Variables|Default|GetBPC_DamageSystem) HealValue))
  (return _newhealth))

(fn IsDead
  (return (Variables|/Game/BP/Components/DamageSystemComponent.DamageSystemComponent_C|GetIsDead (Variables|Default|GetBPC_DamageSystem))))

(fn IsAttacking
  (return (Variables|State|GetAttacking)))

(fn IsCrouching
  (bind _crouching (CallFunction|IsCrouching))
  (return _crouching))

(fn IsRagdoll
  (return false))

(fn OnProjectileHit
  (params (HitLocation :type Vector :default "0, 0, 0") (Attacker :type Actor%20Object%20Reference) (HitNormal :type Vector :default "0, 0, 0"))
  (return false))

(fn ReserveAttackToken
  (params (Amount :type Integer))
  (bind _success (Default|ReserveAttackToken (Variables|Default|GetBPC_DamageSystem) Amount))
  (return _success))

(fn TakeDamage
  (params (DamageInfo :type S%20Damage%20Info%20Structure) (Damage%20Causer :type Actor%20Object%20Reference))
  (if (not (Variables|/Game/BP/Components/AttackComponent.AttackComponent_C|GetIsExecuting (Variables|Default|GetAttackComponent)))
    (bind _wasdamaged (Default|TakeDamage (Variables|Default|GetBPC_DamageSystem) DamageInfo Damage%20Causer))
    (return _wasdamaged)))