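; Interactable loot chest that fills itself with random items and opens its inventory for the player who interacts with it.
; On BeginPlay it creates a lootable inventory widget bound to its InventoryComponent, then builds item objects from random DT_Item rows and tries to add each.
; Item condition is randomized up to the row's value unless that is -1.
; Interaction getters supply the prompt, location, type and hold duration.
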(event Custom|GenerateLoot
  (for _index (range 0 (Math|Random|RandomIntegerinRange 5 20))
    (CallFunction|GetRandomItem)))

(event Custom|GetRandomItem
  (bind _outrownames (DataTable|GetDataTableRowNames "/Game/BP/Inventory/DataTable/DT_Item.DT_Item"))
  (bind _returnvalue (Utilities|GetDataTableRow "/Game/BP/Inventory/DataTable/DT_Item.DT_Item" (.OutItem (Utilities|Array|Random _outrownames)))
    (:then
      (bind _returnvalue_2 (Game|ConstructObjectfromClass "/Game/BP/Interactables/BP_ItemObject.BP_ItemObject_C" (.Dimensions (Utilities|Struct|BreakST_ItemInfo _returnvalue)) (.Icon (Utilities|Struct|BreakST_ItemInfo _returnvalue)) (.IconRotated (Utilities|Struct|BreakST_ItemInfo _returnvalue)) (.ItemClass (Utilities|Struct|BreakST_ItemInfo _returnvalue)) (.ID (Utilities|Struct|BreakST_ItemInfo _returnvalue)) (.Quantity (Utilities|Struct|BreakST_ItemInfo _returnvalue)) (Math|Integer|SelectInt (Math|Random|RandomIntegerinRange 1 (.Condition (Utilities|Struct|BreakST_ItemInfo _returnvalue))) (.Condition (Utilities|Struct|BreakST_ItemInfo _returnvalue)) (!= (.Condition (Utilities|Struct|BreakST_ItemInfo _returnvalue)) -1))))
      (Default|TryAddItem (Variables|Default|GetInventoryComponent) _returnvalue_2))))

(event EventBeginPlay
  (bind _returnvalue (UserInterface|CreateWidget "/Game/BP/Inventory/Widgets/W_InventoryLootable.W_InventoryLootable_C" (Game|GetPlayerController 0) (Variables|Default|GetInventoryComponent) 1e+02))
  (Variables|Default|SetInventoryWidget _returnvalue)
  (CallFunction|GenerateLoot))

(event EventInteract
  (params (Interactor :type Actor%20Object%20Reference))
  (bind _asbp_player_character (Utilities|Casting|CastToBP_PlayerCharacter Interactor))
  (Default|OpenInventory _asbp_player_character (Variables|Default|GetInventoryWidget)))

(fn ConstructionScript)

(fn GetHoldDuration
  (return 1.5))

(fn GetInteractionLocation
  (return (Transformation|GetWorldLocation (Variables|Default|GetInteractionLocation))))

(fn GetInteractionPrompt
  (return "to open chest"))

(fn GetInteractionType
  (return "NewEnumerator1"))

(fn GetTapCount
  (return 0))