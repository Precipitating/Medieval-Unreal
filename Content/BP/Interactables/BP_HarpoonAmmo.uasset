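; Harpoon ammo pickup that players can interact with in the world.
; It supplies the interaction system with a pickup prompt, a world location from its InteractionLocation component, an interaction type and a hold duration.
; Its default item is a BP_ItemObject built from the HarpoonAmmo row of DT_Item, carrying size, icons, class, ID, quantity and condition.
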(fn ConstructionScript
  (|CallParentFunction))

(fn GetInteractionLocation
  (return (Transformation|GetWorldLocation (Variables|Default|GetInteractionLocation))))

(fn GetInteractionPrompt
  (return "to pickup ammo"))

(fn GetDefaultItemObject
  (bind _returnvalue (Utilities|GetDataTableRow "/Game/BP/Inventory/DataTable/DT_Item.DT_Item" "HarpoonAmmo")
    (:then
      (bind _returnvalue_2 (Game|ConstructObjectfromClass self "/Game/BP/Interactables/BP_ItemObject.BP_ItemObject_C" (.Dimensions (Utilities|Struct|BreakST_ItemInfo _returnvalue)) (.Icon (Utilities|Struct|BreakST_ItemInfo _returnvalue)) (.IconRotated (Utilities|Struct|BreakST_ItemInfo _returnvalue)) (.ItemClass (Utilities|Struct|BreakST_ItemInfo _returnvalue)) (.ID (Utilities|Struct|BreakST_ItemInfo _returnvalue)) (.Quantity (Utilities|Struct|BreakST_ItemInfo _returnvalue)) (.Condition (Utilities|Struct|BreakST_ItemInfo _returnvalue))))
      (return _returnvalue_2))))

(fn GetHoldDuration
  (return 1.0))

(fn GetInteractionType
  (return "NewEnumerator1"))