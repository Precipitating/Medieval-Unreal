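; BP_PickUpItem is an interactable world item that the player can pick up into their inventory.
; On BeginPlay it fills a missing ItemObject from GetDefaultItemObject, which returns nothing here.
; Interacting plays a pickup sound, then tries adding the item to the player's InventoryComponent, destroying the actor only on success.
; Getter functions report the interaction type and hold duration, with empty prompt, location and tap count.
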(event EventBeginPlay
  (if (not (Utilities|IsValid (Variables|Private|GetItemObject)))
    (bind _itemobject (Private|GetDefaultItemObject))
    (Variables|Private|SetItemObject _itemobject)))

(event EventInteract
  (params (Interactor :type Actor%20Object%20Reference))
  (Audio|PlaySoundatLocation "/Engine/VREditor/Sounds/UI/Object_PickUp.Object_PickUp" (Transformation|GetWorldLocation (Variables|Default|GetStaticMesh)) "0, 0, 0" 1.0 1.0 0.0 0 0 0 0)
  (bind _asbp_player_character (Utilities|Casting|CastToBP_PlayerCharacter Interactor))
  (bind _added (Default|TryAddItem (Variables|/Game/BP/Player/BP_PlayerCharacter.BP_PlayerCharacter_C|GetInventoryComponent _asbp_player_character) (Variables|Private|GetItemObject)))
  (if _added
    (Actor|DestroyActor)))

(fn ConstructionScript)

(fn GetDefaultItemObject
  (return 0))

(fn GetHoldDuration
  (return (Variables|Default|GetHoldDuration)))

(fn GetInteractionLocation
  (return "0, 0, 0"))

(fn GetInteractionPrompt
  (return ""))

(fn GetInteractionType
  (return "NewEnumerator1"))

(fn GetTapCount
  (return 0))