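; BP_HealthPotObject is an interactable world pickup for the health pot consumable.
; It builds its default BP_ItemObject from the HealthPot row of the DT_Item data table, copying dimensions, icons, class, ID, quantity and condition.
; It also supplies a pick-up prompt and the world position of its InteractionLocation component for interaction.
; The event graph holds only disabled stubs.
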(event EventBeginPlay
  (|CallParentFunction) ; This node is disabled and will not be called.\nDrag off pins to build functionality.
)

(event Collision|EventActorBeginOverlap
  (params (OtherActor :type Actor%20Object%20Reference)))

(event EventTick
  (params (DeltaSeconds :type Float%20%28single-precision%29)))

(fn ConstructionScript
  (|CallParentFunction))

(fn GetDefaultItemObject
  (bind _returnvalue (Utilities|GetDataTableRow "/Game/BP/Inventory/DataTable/DT_Item.DT_Item" "HealthPot")
    (:then
      (bind _returnvalue_2 (Game|ConstructObjectfromClass self "/Game/BP/Interactables/BP_ItemObject.BP_ItemObject_C" (.Dimensions (Utilities|Struct|BreakST_ItemInfo _returnvalue)) (.Icon (Utilities|Struct|BreakST_ItemInfo _returnvalue)) (.IconRotated (Utilities|Struct|BreakST_ItemInfo _returnvalue)) (.ItemClass (Utilities|Struct|BreakST_ItemInfo _returnvalue)) (.ID (Utilities|Struct|BreakST_ItemInfo _returnvalue)) (.Quantity (Utilities|Struct|BreakST_ItemInfo _returnvalue)) (.Condition (Utilities|Struct|BreakST_ItemInfo _returnvalue))))
      (return _returnvalue_2))))

(fn GetInteractionPrompt
  (return "to pick-up consumable"))

(fn GetInteractionLocation
  (return (Transformation|GetWorldLocation (Variables|Default|GetInteractionLocation))))