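; BP_NextRoomDoor is an interactable double door that swings open and closed.
; OpenDoor and CloseDoor play or reverse one Timeline whose yaw drives Door and DoorLeft, with collision disabled on Door during the swing.
; When the Timeline finishes in either direction, it restores collision, clears the Interactor and enables the nav link proxy's smart link.
; TakeDamage always returns false.
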(event EventOpenDoor
  (Variables|Default|SetIsOpen true)
  (Collision|SetCollisionEnabled (Variables|Default|GetDoor) "NoCollision")
  (bind _zrotation (Timeline|Timeline Play)
    (:Update
      (Transformation|SetRelativeRotation (Variables|Default|GetDoor) (Math|Rotator|MakeRotator 0.0 0.0 _zrotation) false false)
      (bind _result (Math|Float|NegateFloat _zrotation)
        (:%20%20
          (Transformation|SetRelativeRotation (Variables|Default|GetDoorLeft) (Math|Rotator|MakeRotator 0.0 0.0 _result) false false))))
    (:Finished
      (Collision|SetCollisionEnabled (Variables|Default|GetDoor) "QueryAndPhysics")
      (Variables|Default|SetInteractor 0)
      (Class|NavLinkProxy|SetSmartLinkEnabled (Variables|Default|GetAs%20Nav%20Link%20Proxy) true))))

(event EventCloseDoor
  (Variables|Default|SetIsOpen false)
  (Collision|SetCollisionEnabled (Variables|Default|GetDoor) "NoCollision")
  (bind _zrotation (Timeline|Timeline Reverse)
    (:Update
      (Transformation|SetRelativeRotation (Variables|Default|GetDoor) (Math|Rotator|MakeRotator 0.0 0.0 _zrotation) false false)
      (bind _result (Math|Float|NegateFloat _zrotation)
        (:%20%20
          (Transformation|SetRelativeRotation (Variables|Default|GetDoorLeft) (Math|Rotator|MakeRotator 0.0 0.0 _result) false false))))
    (:Finished
      (Collision|SetCollisionEnabled (Variables|Default|GetDoor) "QueryAndPhysics")
      (Variables|Default|SetInteractor 0)
      (Class|NavLinkProxy|SetSmartLinkEnabled (Variables|Default|GetAs%20Nav%20Link%20Proxy) true))))

(fn ConstructionScript
  (|CallParentFunction))

(fn TakeDamage
  (params (DamageInfo :type S%20Damage%20Info%20Structure) (Damage%20Causer :type Actor%20Object%20Reference))
  (return false))