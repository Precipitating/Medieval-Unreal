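; Melee enemy Blueprint that fights with a sword, can block incoming damage, and generates sword and health potion loot.
; It spawns its sword on BeginPlay, and montage notifies drive hand attachment and in-use state, with completion reporting equip or unequip.
; Default attacks pass a random slash montage and sword damage info to the attack component.
; TakeDamage attempts a block for blockable hits while armed before forwarding to the damage system, whose blocked event plays a sound.
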(event OnBlocked(BPC_DamageSystem)
  (params (CanBeParried :type Boolean) (DamageInfo :type E_DamageType%20Enum :default "NewEnumerator0") (DamageCauser :type Actor%20Object%20Reference))
  ;[0.15 0.15 0.15 0.5 50] Block sounds
  (switch Utilities|FlowControl|Switch|SwitchonE_DamageType DamageInfo
    (:NewEnumerator2
      (if (Variables|Default|GetIsHoldingWeapon)
        (Audio|PlaySoundatLocation "/Game/Sound/Sword/SwordBlockCue.SwordBlockCue" (Transformation|GetActorLocation) "0, 0, 0" 1.0 1.0 0.0 0 0 0 0)))))

(event Custom|DefaultAttack
  (params (AttackTarget :type Actor%20Object%20Reference))
  ;[0.15 0.15 0.15 0.5 50] Enemy Attacks
  (Default|SwordAttack (Variables|Default|GetAttackComponent) (Utilities|Struct|MakeS_AttackInfo AttackTarget (.OutItem (Utilities|Array|Random (Variables|Default|GetSwordSlashMontage))) (Utilities|Struct|MakeS_DamageInfo 15.0 "NewEnumerator2" "NewEnumerator0" false true true true)) 2e+01 2e+02))

(event EventBeginPlay
  ;[0.15 0.15 0.15 0.5 50] Begin
  (|CallParentFunction)
  (bind _returnvalue (Game|SpawnActorfromClass "/Game/BP/Weapons/BP_Weapon_Sword.BP_Weapon_Sword_C" (Math|Transform|MakeTransform "0, 0, 0" "0, 0, 0" "1.000000,1.000000,1.000000") "Undefined" "MultiplyWithRoot" 0 0))
  (Variables|Default|SetSwordActor _returnvalue))

(event EventEquipWeapon
  (bind _swordactor (Variables|Default|GetSwordActor))
  ;[0.15 0.15 0.15 0.5 50] Enemy Attacks
  (bind _notifyname (Animation|Montage|PlayMontage (Variables|Character|GetMesh) "/Game/Animations/Attacks/Sword/UnSheathingSword_UE_Montage1.UnSheathingSword_UE_Montage1")
    (:OnCompleted
      (Default|CallOnWeaponEquip))
    (:OnNotifyBegin
      (switch name _notifyname
        (:HoldSword
          (Transformation|AttachComponentToComponent _swordactor (Variables|Character|GetMesh) "hand_rSocket" "SnapToTarget" "SnapToTarget" "SnapToTarget" true)
          (Default|SetinUse _swordactor true)
          (Variables|Default|SetIsHoldingWeapon true))))))

(event EventUnEquipWeapon
  ;[0.15 0.15 0.15 0.5 50] Enemy Attacks
  (bind _notifyname (Animation|Montage|PlayMontage (Variables|Character|GetMesh) "/Game/Animations/Attacks/Sword/SheathingSword_UE_Montage.SheathingSword_UE_Montage")
    (:OnCompleted
      (Default|CallOnWeaponUnEquip))
    (:OnNotifyBegin
      (switch name _notifyname
        (:DropSword
          (Default|SetinUse (Variables|Default|GetSwordActor) false)
          (Variables|Default|SetIsHoldingWeapon false))))))

(event EventGenerateLoot
  (CallFunction|SpawnInventoryItem "/Game/BP/Interactables/BP_SwordItem.BP_SwordItem_C" 1)
  (bind _returnvalue (CallFunction|GenerateRandomNumber 1 2))
  (CallFunction|SpawnInventoryItem "/Game/BP/Interactables/BP_HealthPotObject.BP_HealthPotObject_C" _returnvalue))

(fn ConstructionScript
  (|CallParentFunction))

(fn TakeDamage
  (params (DamageInfo :type S%20Damage%20Info%20Structure) (Damage%20Causer :type Actor%20Object%20Reference))
  (if (Utilities|Struct|BreakS_DamageInfo DamageInfo)
    (if (Variables|Default|GetIsHoldingWeapon)
      (CallFunction|AttemptBlock)))
  (bind _wasdamaged (Default|TakeDamage (Variables|Default|GetBPC_DamageSystem) DamageInfo Damage%20Causer))
  (return _wasdamaged))