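; BP_Enemy_Crossbow is a ranged enemy that fights with a crossbow at long attack and defend ranges.
; On BeginPlay it spawns a crossbow actor and attaches it to a hand socket.
; Attacks go through the AttackComponent from spine socket to target and consume ammo, while reloading plays a guarded montage before notifying the weapon.
; It also defines crossbow, ammo and health potion loot, and forwards healing to its damage system.
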(event Custom|DefaultAttack
  (params (AttackTarget :type Actor%20Object%20Reference))
  (Default|CrossbowAttack (Variables|Default|GetAttackComponent) (Utilities|Struct|MakeS_AttackInfo AttackTarget "/Game/Animations/Attacks/Crossbow/FiringRifle_UE_Anim_Montage.FiringRifle_UE_Anim_Montage" (Utilities|Struct|MakeS_DamageInfo 2e+01 "NewEnumerator3" "NewEnumerator0" false false false true)) (Transformation|GetSocketLocation (Variables|Character|GetMesh) "spine_03") (Transformation|GetActorLocation AttackTarget))
  (Default|ConsumeAmmo (Variables|Default|GetWeaponActor)))

(event EventBeginPlay
  (|CallParentFunction)
  (CallFunction|EquipWeapon))

(event EventReload
  (if (not (Variables|Default|GetIsReloading))
    (Variables|Default|SetIsReloading true)
    (Animation|Montage|PlayMontage (Variables|Character|GetMesh) "/Game/Animations/Reload/ModernXbow_Reload_Quiver1_Montage.ModernXbow_Reload_Quiver1_Montage"
      (:OnCompleted
        (Class|BPIWeapon|Reload(Message) (Variables|Default|GetWeaponActor))
        (Variables|Default|SetIsReloading false))
      (:OnInterrupted
        (Variables|Default|SetIsReloading false)))))

(event EventGenerateLoot
  (CallFunction|SpawnInventoryItem "/Game/BP/Interactables/BP_CrossbowItem.BP_CrossbowItem_C" 1)
  (bind _returnvalue (CallFunction|GenerateRandomNumber 1 2))
  (CallFunction|SpawnInventoryItem "/Game/BP/Interactables/BP_CrossbowAmmo.BP_CrossbowAmmo_C" _returnvalue)
  (bind _returnvalue_2 (CallFunction|GenerateRandomNumber 1 2))
  (CallFunction|SpawnInventoryItem "/Game/BP/Interactables/BP_HealthPotObject.BP_HealthPotObject_C" _returnvalue_2))

(event EventEquipWeapon
  (bind _returnvalue (Game|SpawnActorfromClass "/Game/BP/Weapons/BP_Weapon_Crossbow.BP_Weapon_Crossbow_C" (Math|Transform|MakeTransform "0, 0, 0" "0, 0, 0" "1.000000,1.000000,1.000000") "Undefined" "MultiplyWithRoot" 0 0))
  (Default|SetinUse _returnvalue true)
  (bind _output_get (Variables|Default|SetWeaponActor _returnvalue))
  (bind _returnvalue_2 (Transformation|AttachComponentToComponent _output_get (Variables|Character|GetMesh) "hand_rSocket_crossbow" "SnapToTarget" "SnapToTarget" "SnapToTarget" true))
  (Variables|Default|SetIsHoldingWeapon _returnvalue_2)
  (Default|CallOnWeaponEquip))

(fn ConstructionScript
  (|CallParentFunction))

(fn GetIdealRange
  (return 1e+03 6e+02))

(fn Heal
  (params (HealValue :type Float%20%28double-precision%29))
  (bind _newhealth (Default|Heal (Variables|Default|GetBPC_DamageSystem) HealValue))
  (return _newhealth))