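; BP_SpikeTrap is a spike trap that damages actors overlapping its Box.
; The SpikeType enum selects the behavior: activated traps ragdoll the actor through an interface message before the damage message, while static traps skip the ragdoll.
; A successful hit disables damage until a DmgCooldownTime timer re-enables it, with debug prints reporting the cooldown state.
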(event OnComponentBeginOverlap(Box)
  (params (OverlappedComponent :type Primitive%20Component%20Object%20Reference) (OtherActor :type Actor%20Object%20Reference) (OtherComp :type Primitive%20Component%20Object%20Reference) (OtherBodyIndex :type Integer) (bFromSweep :type Boolean) (SweepResult :type Hit%20Result%20Structure%20%28by%20ref%29))
  (if (Variables|Default|GetCanDamage)
    (switch Utilities|FlowControl|Switch|SwitchonTrapType (Variables|Default|GetSpikeType)
      (:NewEnumerator0
        _)
      (:NewEnumerator1
        (Class|BPIDamagable|ApplyRagdoll(Message) OtherActor)))
    (bind _wasdamaged (Class|BPIDamagable|TakeDamage(Message) OtherActor (Utilities|Struct|MakeS_DamageInfo 5.0 "NewEnumerator10")))
    (if _wasdamaged
      (Variables|Default|SetCanDamage false)
      (bind _returnvalue (Utilities|Time|SetTimerbyEvent (delegate Custom|DamageCooldown) (Variables|Default|GetDmgCooldownTime)))
      (Variables|Default|SetDamageCooldownTimer _returnvalue))
    (else
      (Development|PrintString "Spike cooldown"))))

(event Custom|DamageCooldown
  (Variables|Default|SetCanDamage true)
  (Development|PrintString "can damage spikes"))

(fn ConstructionScript)