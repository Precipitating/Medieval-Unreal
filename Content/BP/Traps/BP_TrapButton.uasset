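; BP_TrapButton is an interactable button that activates its linked traps when pressed.
; Interact plays a timeline that pushes the Cube inward, then on completion calls Activate on each linked trap and reverses the timeline, using IsReversing to avoid retriggering.
; A Sphere overlap shows the linked traps' outlines while the player character is nearby.
; Interaction getters supply the prompt and type, with zero hold duration and tap count.
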(event OnComponentBeginOverlap(Sphere)
  (params (OverlappedComponent :type Primitive%20Component%20Object%20Reference) (OtherActor :type Actor%20Object%20Reference) (OtherComp :type Primitive%20Component%20Object%20Reference) (OtherBodyIndex :type Integer) (bFromSweep :type Boolean) (SweepResult :type Hit%20Result%20Structure%20%28by%20ref%29))
  (if (Class|GameplayStatics|ObjectIsA OtherActor "/Game/BP/Player/BP_PlayerCharacter.BP_PlayerCharacter_C")
    (for _array_element (Variables|Default|GetLinkedTrap)
      (Default|SetOutlineVisibility _array_element true))))

(event OnComponentEndOverlap(Sphere)
  (params (OverlappedComponent :type Primitive%20Component%20Object%20Reference) (OtherActor :type Actor%20Object%20Reference) (OtherComp :type Primitive%20Component%20Object%20Reference) (OtherBodyIndex :type Integer))
  (if (Class|GameplayStatics|ObjectIsA OtherActor "/Game/BP/Player/BP_PlayerCharacter.BP_PlayerCharacter_C")
    (for _array_element (Variables|Default|GetLinkedTrap)
      (Default|SetOutlineVisibility _array_element false))))

(event Custom|ReverseButton
  (bind _newtrack_0 (Timeline|ButtonTimeline Reverse)
    (:Update
      (Transformation|SetRelativeLocation (Variables|Default|GetCube) (Math|Vector|MakeVector (Math|Float|Lerp 0.0 -5.0 _newtrack_0) 0.0 0.0) false false))
    (:Finished
      (if (Variables|Default|GetIsReversing)
        (Variables|Default|SetIsReversing false)
        (else
          (Variables|Default|SetIsReversing true)
          (CallFunction|ActivateTraps)
          (CallFunction|ReverseButton))))))

(event Custom|ActivateTraps
  (for _array_element (Variables|Default|GetLinkedTrap)
    (Default|Activate _array_element)))

(event EventInteract
  (params (Interactor :type Actor%20Object%20Reference))
  (bind _newtrack_0 (Timeline|ButtonTimeline Play)
    (:Update
      (Transformation|SetRelativeLocation (Variables|Default|GetCube) (Math|Vector|MakeVector (Math|Float|Lerp 0.0 -5.0 _newtrack_0) 0.0 0.0) false false))
    (:Finished
      (if (Variables|Default|GetIsReversing)
        (Variables|Default|SetIsReversing false)
        (else
          (Variables|Default|SetIsReversing true)
          (CallFunction|ActivateTraps)
          (CallFunction|ReverseButton))))))

(event EventSetLinkedTrap
  (params (Trap :type Array%20of%20BP%20Trap%20Base%20Object%20References))
  (Variables|Default|SetLinkedTrap Trap))

(fn ConstructionScript)

(fn GetHoldDuration
  (return 0.0))

(fn GetInteractionLocation
  (return "0, 0, 0"))

(fn GetInteractionPrompt
  (return "to activate trap"))

(fn GetInteractionType
  (return "NewEnumerator0"))

(fn GetLinkedTrap
  (return 0))

(fn GetTapCount
  (return 0))