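; BP_Spike is a trap that impales ragdolled actors on its cone and deals massive damage.
; When the cone is overlapped, it line-traces along its up vector for a randomized, scale-adjusted length.
; If the actor reports ragdoll and a bone is hit, a physics constraint pins that bone to the cone and damage is sent by message.
; Debug trace drawing and bone-name printing remain active; a multi-trace loop is unused.
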(event OnComponentBeginOverlap(Cone)
  (params (OverlappedComponent :type Primitive%20Component%20Object%20Reference) (OtherActor :type Actor%20Object%20Reference) (OtherComp :type Primitive%20Component%20Object%20Reference) (OtherBodyIndex :type Integer) (bFromSweep :type Boolean) (SweepResult :type Hit%20Result%20Structure%20%28by%20ref%29))
  (bind _defaultsceneroot (Variables|Default|GetDefaultSceneRoot))
  (bind _cone (Variables|Default|GetCone))
  (bind _returnvalue (Transformation|GetWorldLocation _defaultsceneroot))
  (bind _outhit (Collision|LineTraceByChannel _returnvalue (+ _returnvalue (* (Math|Vector|GetUpVector _cone) (* (Math|Random|RandomIntegerinRange 85 100) (.z (Transformation|GetWorldScale _cone))))) "TraceTypeQuery1" false 0 "ForDuration"))
  (bind _returnvalue_2 (Class|BPIDamagable|IsRagdoll(Message) OtherActor))
  (if _returnvalue_2
    (if (!= (.hitbonename _outhit) "")
      (Development|PrintString (Utilities|String|ToString(Name) (.hitbonename _outhit)))
      (Class|PhysicsConstraintComponent|SetConstrainedComponents (Variables|Default|GetPhysicsConstraint) (Variables|Default|GetCone) "None" (.hitcomponent _outhit) (.hitbonename _outhit))
      (Class|BPIDamagable|TakeDamage(Message) OtherActor (Utilities|Struct|MakeS_DamageInfo 999.0 "NewEnumerator10" "NewEnumerator1")))))

(fn ConstructionScript)