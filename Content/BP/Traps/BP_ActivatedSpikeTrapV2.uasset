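; An activated spike trap that extends its Plane component along local Y by ExtendLength when triggered, then retracts.
; Activate plays a timeline that lerps the plane's offset, and its completion calls Reset to reverse the timeline.
; The construction script sizes a two-point spline to ExtendLength and builds a spline mesh along it as TrapOutlineMesh.
; That mesh's visibility is switchable, and overlaps toggle its custom depth stencil value.
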(event OnComponentBeginOverlap(TrapOutlineMesh)
  (params (OverlappedComponent :type Primitive%20Component%20Object%20Reference) (OtherActor :type Actor%20Object%20Reference) (OtherComp :type Primitive%20Component%20Object%20Reference) (OtherBodyIndex :type Integer) (bFromSweep :type Boolean) (SweepResult :type Hit%20Result%20Structure%20%28by%20ref%29))
  (Rendering|SetCustomDepthStencilValue (Variables|Default|GetTrapOutlineMesh) 2))

(event OnComponentEndOverlap(TrapOutlineMesh)
  (params (OverlappedComponent :type Primitive%20Component%20Object%20Reference) (OtherActor :type Actor%20Object%20Reference) (OtherComp :type Primitive%20Component%20Object%20Reference) (OtherBodyIndex :type Integer))
  (Rendering|SetCustomDepthStencilValue (Variables|Default|GetTrapOutlineMesh) 0))

(event Custom|Reset
  (bind _newtrack_0 (Timeline|Timeline Reverse)
    (:Update
      (Transformation|SetRelativeLocation (Variables|Default|GetPlane) (Math|Vector|MakeVector 0.0 (Math|Float|Lerp 0.0 (Variables|Default|GetExtendLength) _newtrack_0) 0.0) false false))
    (:Finished
      (CallFunction|Reset))))

(event EventBeginPlay
  (|CallParentFunction) ; This node is disabled and will not be called.\nDrag off pins to build functionality.
)

(event Collision|EventActorBeginOverlap
  (params (OtherActor :type Actor%20Object%20Reference))
  (|CallParentFunction OtherActor) ; This node is disabled and will not be called.\nDrag off pins to build functionality.
)

(event EventTick
  (params (DeltaSeconds :type Float%20%28single-precision%29))
  (|CallParentFunction DeltaSeconds) ; This node is disabled and will not be called.\nDrag off pins to build functionality.
)

(event EventActivate
  (bind _newtrack_0 (Timeline|Timeline Play)
    (:Update
      (Transformation|SetRelativeLocation (Variables|Default|GetPlane) (Math|Vector|MakeVector 0.0 (Math|Float|Lerp 0.0 (Variables|Default|GetExtendLength) _newtrack_0) 0.0) false false))
    (:Finished
      (CallFunction|Reset))))

(event EventSetOutlineVisibility
  (params (On :type Boolean))
  (Rendering|SetVisibility (Variables|Default|GetTrapOutlineMesh) On false))

(fn ConstructionScript
  (bind _extendlengthspline (Variables|Default|GetExtendLengthSpline))
  (bind _extendlengthspline_2 (Variables|Default|GetExtendLengthSpline))
  (|CallParentFunction)
  (Spline|SetLocationatSplinePoint (Variables|Default|GetExtendLengthSpline) 1 (+ (Spline|GetLocationatSplinePoint (Variables|Default|GetExtendLengthSpline) 0 "Local") (Math|Vector|MakeVector 0.0 (Variables|Default|GetExtendLength) 0.0)) "Local" true)
  (bind _returnvalue (AddComponent|AddSplineMeshComponent false (Math|Transform|MakeTransform "0, 0, 0" "0, 0, 0" (Variables|Default|GetRelative%20Transform%20Scale))))
  (Variables|Default|SetTrapOutlineMesh _returnvalue)
  (SplineMesh|SetForwardAxis (Variables|Default|GetTrapOutlineMesh) "Y" true)
  (SplineMesh|SetStartandEnd (Variables|Default|GetTrapOutlineMesh) (Spline|GetLocationatSplinePoint _extendlengthspline 0 "Local") (Spline|GetTangentatSplinePoint _extendlengthspline 0 "Local") (Spline|GetLocationatSplinePoint _extendlengthspline_2 1 "Local") (Spline|GetTangentatSplinePoint _extendlengthspline_2 1 "Local") true :!class /Script/Engine.SplineMeshComponent))