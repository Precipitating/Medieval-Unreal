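; Spike trap that damages, ragdolls or instantly kills actors according to its SpikeType.
; On BeginPlay it binds hit events on the meshes nested under SpikeList.
; Hitting an already ragdolled actor's bone kills it, impales it through a spawned PhysicsControlActor, unbinds that spike and spawns pooled blood.
; A base overlap fallback catches missed spikes, and a cooldown timer throttles non-lethal damage.
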(event OnComponentBeginOverlap(BaseCollision)
  (params (OverlappedComponent :type Primitive%20Component%20Object%20Reference) (OtherActor :type Actor%20Object%20Reference) (OtherComp :type Primitive%20Component%20Object%20Reference) (OtherBodyIndex :type Integer) (bFromSweep :type Boolean) (SweepResult :type Hit%20Result%20Structure%20%28by%20ref%29))
  ;[0.15 0.15 0.15 0.5 30] Incase pawn doesn't hit the spike but the base of the trap
  (switch Utilities|FlowControl|Switch|SwitchonTrapType (Variables|Default|GetSpikeType)
    (:NewEnumerator0
      (if (Variables|Default|GetCanDamage)
        (bind _wasdamaged (Class|BPIDamagable|TakeDamage(Message) OtherActor (Utilities|Struct|MakeS_DamageInfo 5.0 "NewEnumerator10")))
        (if _wasdamaged
          (Variables|Default|SetCanDamage false)
          (bind _returnvalue (Utilities|Time|SetTimerbyEvent (delegate Custom|DamageCooldown) (Variables|Default|GetDmgCooldownTime)))
          (Variables|Default|SetDamage%20Cooldown%20Timer _returnvalue))))
    (:NewEnumerator1
      (Class|BPIDamagable|ApplyRagdoll(Message) OtherActor))
    (:NewEnumerator2
      (Class|BPIDamagable|TakeDamage(Message) OtherActor (Utilities|Struct|MakeS_DamageInfo 999.0 "NewEnumerator10")))))

(event Custom|BindOverlapBegin
  ;[0.15 0.15 0.15 0.5 30] Impale logic
  (for _array_element (Components|GetChildrenComponents (Variables|Default|GetSpikeList) false)
    (for _array_element_2 (Components|GetChildrenComponents _array_element false)
      (bind _asstatic_mesh_component (Utilities|Casting|CastToStaticMeshComponent _array_element_2))
      (Collision|BindEventtoOnComponentHit _asstatic_mesh_component (delegate Custom|SpikeHandler)))))

(event Custom|SpikeHandler
  (params (HitComponent :type Primitive%20Component%20Object%20Reference) (OtherActor :type Actor%20Object%20Reference) (OtherComp :type Primitive%20Component%20Object%20Reference) (NormalImpulse :type Vector) (Hit :type Hit%20Result%20Structure%20%28by%20ref%29))
  (bind _returnvalue (Math|Conversions|ToTransform(Vector) (.impactpoint Hit)))
  ;[0.15 0.15 0.15 0.5 30] Impale logic
  (bind _returnvalue_2 (Class|BPIDamagable|IsRagdoll(Message) OtherActor))
  (if _returnvalue_2
    (if (!= (.hitbonename Hit) "")
      (Development|PrintString (Utilities|String|ToString(Name) (.hitbonename Hit)))
      (bind _returnvalue_3 (Game|SpawnActorfromClass "/Script/PhysicsControl.PhysicsControlActor" _returnvalue "AlwaysSpawn" "MultiplyWithRoot" 0 0))
      (Class|BPIDamagable|TakeDamage(Message) OtherActor (Utilities|Struct|MakeS_DamageInfo 999.0 "NewEnumerator10" "NewEnumerator1" false false false true))
      (Class|PhysicsControlComponent|CreateControl :self (Variables|/Script/PhysicsControl.PhysicsControlActor|GetControlComponent _returnvalue_3) :ParentComponent HitComponent :ChildComponent (.hitcomponent Hit) :ChildBoneName (.hitbonename Hit) :ControlData (Utilities|Struct|MakePhysicsControlData 1e+01 1.0 0.0 0.0 1e+01 1.0 0.0 0.0 1.0 1.0 1.0 "0.000000,0.000000,0.000000" true false false))
      (Collision|UnbindEventfromOnComponentHit HitComponent (delegate Custom|SpikeHandler))
      (bind _asdefault_game_mode (Utilities|Casting|CastToDefaultGameMode (Game|GetGameMode)))
      (Default|SpawnfromPool (Variables|/Game/DefaultGameMode.DefaultGameMode_C|GetSwordSlashBloodPool _asdefault_game_mode) _returnvalue))
    (else
      (switch Utilities|FlowControl|Switch|SwitchonTrapType (Variables|Default|GetSpikeType)
        (:NewEnumerator0
          (if (Variables|Default|GetCanDamage) :!label _label
            (bind _wasdamaged (Class|BPIDamagable|TakeDamage(Message) OtherActor (Utilities|Struct|MakeS_DamageInfo 5.0 "NewEnumerator10")))
            (if _wasdamaged
              (Variables|Default|SetCanDamage false)
              (bind _returnvalue_4 (Utilities|Time|SetTimerbyEvent (delegate Custom|DamageCooldown) (Variables|Default|GetDmgCooldownTime)))
              (Variables|Default|SetDamage%20Cooldown%20Timer _returnvalue_4))))
        (:NewEnumerator1
          (Class|BPIDamagable|ApplyRagdoll(Message) OtherActor)
          (goto _label))
        (:NewEnumerator2
          (Class|BPIDamagable|TakeDamage(Message) OtherActor (Utilities|Struct|MakeS_DamageInfo 999.0 "NewEnumerator10")))))))

(event Custom|DamageCooldown
  ;[0.15 0.15 0.15 0.5 30] Impale logic
  (Variables|Default|SetCanDamage true)
  (Development|PrintString "can damage spikes"))

(event EventBeginPlay
  (|CallParentFunction)
  (CallFunction|BindOverlapBegin))

(fn ConstructionScript
  (|CallParentFunction))