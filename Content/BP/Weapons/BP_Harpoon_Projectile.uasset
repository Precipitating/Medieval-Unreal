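; Harpoon projectile with an in-use toggle that launches it along its mesh's forward vector or detaches and halts it.
; Box overlaps damage characters on other teams, while non-character hits stop it in place.
; A successful harpoon hit spawns pooled blood, then traces forward and spawns a BP_SurfacePinner.
; The pinner's two physics constraints attach to the static world and the hit physics body's bone, pinning bodies to surfaces.
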(event OnComponentBeginOverlap(Box)
  (params (OverlappedComponent :type Primitive%20Component%20Object%20Reference) (OtherActor :type Actor%20Object%20Reference) (OtherComp :type Primitive%20Component%20Object%20Reference) (OtherBodyIndex :type Integer) (bFromSweep :type Boolean) (SweepResult :type Hit%20Result%20Structure%20%28by%20ref%29))
  (bind _projectilemovement (Variables|Default|GetProjectileMovement))
  (bind _staticmesh (Variables|Default|GetStaticMesh))
  (bind _returnvalue (Transformation|GetWorldLocation _staticmesh))
  (if (!= OtherActor (stale EventSetinUse Owner))
    (Class|KismetSystemLibrary|IsObjectOfSoftClass OtherActor "/Script/Engine.Character"
      (:True
        (bind _teamnumber (Class|BPIDamagable|GetTeamNumber(Message) (stale EventSetinUse Owner)))
        (bind _teamnumber_2 (Class|BPIDamagable|GetTeamNumber(Message) OtherActor))
        (if (!= _teamnumber _teamnumber_2)
          (bind _wasdamaged (Class|BPIDamagable|TakeDamage(Message) OtherActor (stale EventSetinUse DamageInfo) (stale EventSetinUse Owner)))
          (if _wasdamaged
            (switch Utilities|FlowControl|Switch|SwitchonE_DamageType (.DamageType (Utilities|Struct|BreakS_DamageInfo (stale EventSetinUse DamageInfo)))
              (:NewEnumerator11
                ;[0.15 0.15 0.15 0.5] Blood splatter on hit location (bolt)
                (bind _asdefault_game_mode (Utilities|Casting|CastToDefaultGameMode (Game|GetGameMode)))
                (Default|SpawnfromPool (Variables|/Game/DefaultGameMode.DefaultGameMode_C|GetCrossbowBloodPool _asdefault_game_mode) (Transformation|GetWorldTransform (Variables|Default|GetBox)))
                ;[0.15 0.15 0.15 0.5] Surface Pin
                (bind _outhits (Class|KismetSystemLibrary|LineTraceMultiforObjects _returnvalue (+ _returnvalue (* (Math|Vector|GetForwardVector (Transformation|GetWorldRotation _staticmesh)) 1e+03)) (Utilities|Array|MakeArray "ObjectTypeQuery1" "ObjectTypeQuery4") false 0 "None" true))
                (if (>= (Utilities|Array|Length _outhits) 2)
                  (bind _returnvalue_2 (Game|SpawnActorfromClass "/Game/BP/Weapons/BP_SurfacePinner.BP_SurfacePinner_C" (Math|Transform|MakeTransform "0, 0, 0" "0, 0, 0" "1.000000,1.000000,1.000000") "Undefined" "MultiplyWithRoot" 0 0))
                  (Variables|Default|SetPin _returnvalue_2)
                  (bind _arrayelement (Utilities|Array|ReverseforEachLoop _outhits)
                    (:LoopBody
                      (switch Utilities|FlowControl|Switch|SwitchonECollisionChannel (Collision|GetCollisionObjectType (.HitComponent (Collision|BreakHitResult _arrayelement)))
                        (:ECC_WorldStatic
                          (Utilities|FlowControl|DoOnce false
                            (:Completed
                              (Transformation|SetWorldLocation (Variables|/Game/BP/Weapons/BP_SurfacePinner.BP_SurfacePinner_C|GetSphereA (Variables|Default|GetPin)) (.ImpactPoint (Collision|BreakHitResult _arrayelement)) false false)
                              (Class|PhysicsConstraintComponent|SetConstrainedComponents (Variables|/Game/BP/Weapons/BP_SurfacePinner.BP_SurfacePinner_C|GetPhysicsConstraintA (Variables|Default|GetPin)) (Variables|/Game/BP/Weapons/BP_SurfacePinner.BP_SurfacePinner_C|GetSphereA (Variables|Default|GetPin)) "None" (.HitComponent (Collision|BreakHitResult _arrayelement)) "None"))))
                        (:ECC_PhysicsBody
                          (Utilities|FlowControl|DoOnce false
                            (:Completed
                              (Transformation|SetWorldLocation (Variables|/Game/BP/Weapons/BP_SurfacePinner.BP_SurfacePinner_C|GetSphereB (Variables|Default|GetPin)) (.ImpactPoint (Collision|BreakHitResult _arrayelement)) false false)
                              (Class|PhysicsConstraintComponent|SetConstrainedComponents (Variables|/Game/BP/Weapons/BP_SurfacePinner.BP_SurfacePinner_C|GetPhysicsConstraintB (Variables|Default|GetPin)) (Variables|/Game/BP/Weapons/BP_SurfacePinner.BP_SurfacePinner_C|GetSphereB (Variables|Default|GetPin)) "None" (.HitComponent (Collision|BreakHitResult _arrayelement)) (.HitBoneName (Collision|BreakHitResult _arrayelement))))))))))))
            (else
              (Development|PrintString "NO HIT")))))
      (:False
        (Components|Movement|StopMovementImmediately _projectilemovement)
        (Variables|/Script/Engine.ProjectileMovementComponent|SetProjectileGravityScale _projectilemovement 0.0)))))

(event EventSetinUse
  (params (InUse :type Boolean) (Owner :type Actor%20Object%20Reference) (DamageInfo :type S%20Damage%20Info%20Structure))
  (|CallParentFunction InUse Owner DamageInfo)
  (if InUse
    (Components|Tick|SetComponentTickEnabled (Variables|Default|GetProjectileMovement) true)
    (Variables|/Script/Engine.MovementComponent|SetVelocity (Variables|Default|GetProjectileMovement) (* (Math|Vector|GetForwardVector (Variables|Default|GetStaticMesh)) (Variables|Default|GetSpeed)))
    (Variables|/Script/Engine.ProjectileMovementComponent|SetProjectileGravityScale (Variables|Default|GetProjectileMovement) (Variables|Default|GetGravityScale))
    (else
      (Components|Tick|SetComponentTickEnabled (Variables|Default|GetProjectileMovement) false)
      (Transformation|DetachFromActor "KeepRelative" "KeepRelative" "KeepRelative")
      (Components|Movement|StopMovementImmediately (Variables|Default|GetProjectileMovement)))))

(fn ConstructionScript)