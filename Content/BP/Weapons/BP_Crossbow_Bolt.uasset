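; Pooled crossbow bolt that launches forward under projectile movement when set in use, and detaches and stops when released.
; Box overlaps damage characters on other teams through interface messages; successful Bolt hits spawn pooled blood, release the bolt and report the hit to the victim.
; Overlapping non-characters freezes the bolt in place.
; A separate SpawnBoltProjectile function, not called here, interpolates the bolt along precomputed arc points, releasing it afterwards.
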(event OnComponentBeginOverlap(Box)
  (params (OverlappedComponent :type Primitive%20Component%20Object%20Reference) (OtherActor :type Actor%20Object%20Reference) (OtherComp :type Primitive%20Component%20Object%20Reference) (OtherBodyIndex :type Integer) (bFromSweep :type Boolean) (SweepResult :type Hit%20Result%20Structure%20%28by%20ref%29))
  (bind _projectilemovement (Variables|Default|GetProjectileMovement))
  (if (!= OtherActor (stale EventSetinUse Owner))
    (Class|KismetSystemLibrary|IsObjectOfSoftClass OtherActor "/Script/Engine.Character"
      (:True
        (bind _teamnumber (Class|BPIDamagable|GetTeamNumber(Message) (stale EventSetinUse Owner)))
        (bind _teamnumber_2 (Class|BPIDamagable|GetTeamNumber(Message) OtherActor))
        (if (!= _teamnumber _teamnumber_2)
          (bind _wasdamaged (Class|BPIDamagable|TakeDamage(Message) OtherActor (stale EventSetinUse DamageInfo) (stale EventSetinUse Owner)))
          (if _wasdamaged
            (switch Utilities|FlowControl|Switch|SwitchonE_DamageType (.DamageType (Utilities|Struct|BreakS_DamageInfo (stale EventSetinUse DamageInfo)))
              (:NewEnumerator3
                ;[0.15 0.15 0.15 0.5] Blood splatter on hit location (bolt)
                (bind _asdefault_game_mode (Utilities|Casting|CastToDefaultGameMode (Game|GetGameMode)))
                (Default|SpawnfromPool (Variables|/Game/DefaultGameMode.DefaultGameMode_C|GetCrossbowBloodPool _asdefault_game_mode) (Transformation|GetWorldTransform (Variables|Default|GetBox)))
                (CallFunction|SetinUse false)
                ;[0.15 0.15 0.15 0.5] Attach bolt to actor
                (Class|BPIDamagable|OnProjectileHit(Message) OtherActor (Transformation|GetWorldLocation (Variables|Default|GetBox)) 0 (Math|Vector|GetForwardVector (Variables|Default|GetStaticMesh)))))
            (else
              (Development|PrintString "NO HIT")))))
      (:False
        (Components|Movement|StopMovementImmediately _projectilemovement)
        (Variables|/Script/Engine.ProjectileMovementComponent|SetProjectileGravityScale _projectilemovement 0.0)))))

(event EventSetinUse
  (params (InUse :type Boolean) (Owner :type Actor%20Object%20Reference) (DamageInfo :type S%20Damage%20Info%20Structure))
  (|CallParentFunction InUse Owner DamageInfo)
  (if InUse
    (Components|Tick|SetComponentTickEnabled (Variables|Default|GetProjectileMovement) true)
    (Variables|/Script/Engine.MovementComponent|SetVelocity (Variables|Default|GetProjectileMovement) (* (Math|Vector|GetForwardVector (Variables|Default|GetStaticMesh)) (Variables|Default|GetSpeed)))
    (Variables|/Script/Engine.ProjectileMovementComponent|SetProjectileGravityScale (Variables|Default|GetProjectileMovement) (Variables|Default|GetGravityScale))
    (else
      (Components|Tick|SetComponentTickEnabled (Variables|Default|GetProjectileMovement) false)
      (Transformation|DetachFromActor "KeepRelative" "KeepRelative" "KeepRelative")
      (Components|Movement|StopMovementImmediately (Variables|Default|GetProjectileMovement)))))

(fn ConstructionScript)

(fn SpawnBoltProjectile
  (params (Delta :type Float%20%28double-precision%29))
  (if (and (Utilities|Array|IsNotEmpty (Variables|Default|GetArcPositions)) (< (Variables|Default|GetCurrentArcIdx) (Utilities|Array|Length (Variables|Default|GetArcPositions))))
    (Transformation|SetActorLocation (Math|Interpolation|VInterpTo (Transformation|GetActorLocation) (Utilities|Array|Get(acopy) (Variables|Default|GetArcPositions) (Variables|Default|GetCurrentArcIdx)) Delta 3e+01) false false)
    (if (and (> (Variables|Default|GetCurrentArcIdx) 0) (< (+ (Variables|Default|GetCurrentArcIdx) 1) (Utilities|Array|Length (Variables|Default|GetArcPositions))))
      (Transformation|SetActorRotation (Math|Rotator|FindLookatRotation (Utilities|Array|Get(acopy) (Variables|Default|GetArcPositions) (Variables|Default|GetCurrentArcIdx)) (Utilities|Array|Get(acopy) (Variables|Default|GetArcPositions) (+ (Variables|Default|GetCurrentArcIdx) 1)))))
    (if (< (Math|Vector|Distance(Vector) (Transformation|GetActorLocation) (Utilities|Array|Get(acopy) (Variables|Default|GetArcPositions) (Variables|Default|GetCurrentArcIdx))) 1e+01)
      (Math|Integer|IncrementInt (Variables|Default|GetCurrentArcIdx)))
    (else
      (CallFunction|SetinUse false))))