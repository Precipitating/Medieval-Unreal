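; Base weapon actor that manages in-use state and ammo, showing the count on an attached widget.
; It starts not in use; SetInUse toggles collision and visibility, with tick enabled only while not in use.
; ConsumeAmmo subtracts the per-shot cost and Reload refills to max, both refreshing the widget.
; Getters expose state and reload need, and weapons without ammo hide the counter on BeginPlay.
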(event Custom|SetInUse
  (params (InUse :type Boolean))
  (bind _returnvalue (not InUse))
  (Variables|Default|SetInUse InUse)
  (Collision|SetActorEnableCollision InUse)
  (Rendering|SetActorHiddenInGame _returnvalue)
  (Actor|Tick|SetActorTickEnabled _returnvalue))

(event EventReload
  (bind _output_get (Variables|Default|SetAmmo (Variables|Default|GetMaxAmmo)))
  (Default|UpdateAmmoCount (Variables|Default|GetWidgetRef) _output_get (Variables|Default|GetMaxAmmo)))

(event EventConsumeAmmo
  (if (> (Variables|Default|GetAmmo) 0)
    (bind _output_get (Variables|Default|SetAmmo (- (Variables|Default|GetAmmo) (Variables|Default|GetAmmoCostPerShot))))
    (Default|UpdateAmmoCount (Variables|Default|GetWidgetRef) _output_get (Variables|Default|GetMaxAmmo))))

(event EventBeginPlay
  (CallFunction|SetinUse false)
  (bind _result (CallFunction|WeaponUsesAmmo))
  (bind _asw_ammo_count (Utilities|Casting|CastToW_AmmoCount (UserInterface|GetUserWidgetObject (Variables|Default|GetAmmoWidget))))
  (bind _output_get (Variables|Default|SetWidgetRef _asw_ammo_count))
  (if _result
    (bind _getammo (CallFunction|GetAmmo))
    (Default|UpdateAmmoCount _output_get _getammo (Variables|Default|GetMaxAmmo))
    (else
      (Default|SetVisible _output_get false))))

(fn ConstructionScript)

(fn IsinUse
  (return (Variables|Default|GetInUse)))

(fn GetAmmo
  (return (Variables|Default|GetAmmo)))

(fn GetAmmoCostPerShot
  (return (Variables|Default|GetAmmoCostPerShot)))

(fn GetMaxAmmo
  (return (Variables|Default|GetMaxAmmo)))

(fn NeedsReload
  (return (<= (Variables|Default|GetAmmo) 0)))

(fn WeaponUsesAmmo
  (return (Variables|Default|GetWeaponRequiresAmmo)))