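; BP_Master is a dungeon Blueprint that provides helper functions for wiring buttons to traps built as child actor components.
; GetMultipleTrapsArray gathers the direct child actor components under a given parent component.
; LinkButtonToTrap reads each trap's linked-trap message from its child actor, collects them into an array and passes it to the button's child actor.
; The event graph and construction script do nothing, and neither helper is called here.
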(event EventBeginPlay)

(event Collision|EventActorBeginOverlap
  (params (OtherActor :type Actor%20Object%20Reference)))

(event EventTick
  (params (DeltaSeconds :type Float%20%28single-precision%29)))

(fn ConstructionScript)

(fn LinkButtontoTrap
  (params (Button :type Child%20Actor%20Component%20Object%20Reference) (Traps :type Array%20of%20Child%20Actor%20Component%20Object%20References))
  (for _array_element Traps
    (bind _trap (Class|BPILinkedTrap|GetLinkedTrap(Message) (Variables|/Script/Engine.ChildActorComponent|GetChildActor _array_element)))
    (Utilities|Array|Add (LocalVariables|GetTrapArray) _trap))
  (Class|BPILinkedTrap|SetLinkedTrap(Message) (Variables|/Script/Engine.ChildActorComponent|GetChildActor Button) (LocalVariables|GetTrapArray)))

(fn GetMultipleTrapsArray
  (params (Parent :type Scene%20Component%20Object%20Reference))
  (for _array_element (Components|GetChildrenComponents Parent false)
    (bind _aschild_actor_component (Utilities|Casting|CastToChildActorComponent _array_element))
    (Utilities|Array|Add (LocalVariables|GetResult) _aschild_actor_component))
  (return (LocalVariables|GetResult)))