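; Reusable bloodstain actor that shows an animated blood decal whenever it is set in use.
; After calling the parent and briefly waiting, it creates a dynamic instance of the Plane's material and shares it with the Decal.
; One timeline drives Opening_Rate to open the stain; after Lifetime, a second drives the "qq" parameter to dissolve it.
; When dissolving finishes, the actor sets itself out of use.
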(event EventSetinUse
  (params (InUse :type Boolean) (Owner :type Actor%20Object%20Reference) (DamageInfo :type S%20Damage%20Info%20Structure))
  (bind _plane (Variables|Default|GetPlane))
  (bind _returnvalue (Rendering|Material|GetMaterial _plane 0))
  (|CallParentFunction InUse 0 "")
  (if InUse
    (Utilities|FlowControl|Delay 0.1)
    (Variables|Default|SetStatic_Material _returnvalue)
    (Rendering|Components|Decal|SetDecalMaterial (Variables|Default|GetDecal) _returnvalue)
    (bind _returnvalue_2 (Rendering|Material|CreateDynamicMaterialInstance (Variables|Default|GetPlane) 0 (Variables|Default|GetStatic_Material) "None" :!class /Script/Engine.PrimitiveComponent))
    (bind _output_get (Variables|Default|SetMaterial _returnvalue_2))
    (Rendering|Components|Decal|SetDecalMaterial (Variables|Default|GetDecal) _returnvalue_2)
    (bind _dissolve_rate (Timeline|Timeline_0 Play)
      (:Update
        (Rendering|Material|SetScalarParameterValue _output_get "Opening_Rate" _dissolve_rate :!class /Script/Engine.MaterialInstanceDynamic))
      (:Finished
        (Utilities|FlowControl|Delay (Variables|Default|GetLifetime))
        (bind _dissolve_rate_2 (Timeline|Dissolving Play)
          (:Update
            (Rendering|Material|SetScalarParameterValue _returnvalue_2 "qq" _dissolve_rate_2 :!class /Script/Engine.MaterialInstanceDynamic))
          (:Finished
            (CallFunction|SetinUse false)))))))

(fn ConstructionScript)