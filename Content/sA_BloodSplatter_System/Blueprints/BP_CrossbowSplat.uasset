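; BP_CrossbowSplat is a pooled blood splatter effect, named for crossbow hits, that sprays droplets and leaves stains.
; On BeginPlay it configures a Niagara burst with size, speed, gravity, count and color, and SetinUse toggles it.
; Niagara's particle-data callback pulls BP_Bloodstain_Main actors from the GameMode's pool at particle positions, oriented by velocity.
; Stains get randomized scale, yaw and material, plus the color and lifetime.
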(event Custom|SpawnDrops
  (bind _dropletstyle_niagara (Variables|Default|GetDropletStyle_Niagara))
  (bind _particle_maxdistance (Variables|Droplet_Options|GetParticle_MaxDistance))
  (bind _dropletstyle_niagara_2 (Variables|Default|GetDropletStyle_Niagara))
  ;[0 0.02129 1] SPAWN DROPs
  (Class|NiagaraComponent|SetAsset _dropletstyle_niagara_2 (Variables|Droplet_Options|GetBurst_Style) true)
  (Niagara|SetNiagaraVariable(Float) _dropletstyle_niagara_2 "Gravity_Scale" (Variables|Droplet_Options|GetGravity_Scale))
  (Niagara|SetNiagaraVariable(Float) _dropletstyle_niagara_2 "SpeetMultiplier_Max" _particle_maxdistance)
  (Niagara|SetNiagaraVariable(Float) _dropletstyle_niagara_2 "Dist" (+ (Variables|Droplet_Options|GetParticle_LifeTime_Multiplier) _particle_maxdistance))
  (Niagara|SetNiagaraVariable(Float) _dropletstyle_niagara_2 "SpeedMultiplier" (Variables|Droplet_Options|GetParticle_Min_Distance))
  (Niagara|SetNiagaraVariable(Float) _dropletstyle_niagara_2 "Particle_Sizew" (Variables|Droplet_Options|GetParticle_Size))
  (Class|NiagaraComponent|SetVariableInt _dropletstyle_niagara_2 "Spawn_Rate" (Variables|Droplet_Options|GetMax_Drops))
  (Niagara|SetNiagaraVariable(Object) _dropletstyle_niagara "User.BP_CallBack" self)
  (Niagara|SetNiagaraVariable(LinearColor) _dropletstyle_niagara "Color" (Variables|Default|GetColor)))

(event EventParticleData
  (params (Data :type Array%20of%20Basic%20Particle%20Data%20Structures) (NiagaraSystem :type Niagara%20System%20Object%20Reference) (SimulationPositionOffset :type Vector%20%28by%20ref%29 :default "0, 0, 0"))
  (bind _splat_materials (Variables|Splat_Options|GetSplat_Materials))
  ;[1 0.2708 0.7189] SPLAT SPAWN
  (bind _asdefault_game_mode (Utilities|Casting|CastToDefaultGameMode (Game|GetGameMode)))
  (bind _pooledactor (Default|SpawnfromPool (Variables|/Game/DefaultGameMode.DefaultGameMode_C|GetMainBloodParticlePool _asdefault_game_mode) (Math|Transform|MakeTransform (.Position (Utilities|Struct|BreakBasicParticleData (stale _array_element))) (Math|Rotator|MakeRotfromZ (.Velocity (Utilities|Struct|BreakBasicParticleData (stale _array_element)))) (Math|Conversions|ToVector(Float) (/ (Math|Random|RandomFloatinRange (Variables|Splat_Options|GetSplatSize_Min) (Variables|Splat_Options|GetSplatSize_Max)) (Math|Float|Clamp(Float) (/ (Math|Float|Clamp(Float) (.Size (Utilities|Struct|BreakBasicParticleData (stale _array_element))) 1e+02 1e+03) 1e+02) 1.0 (* (Math|Float|Clamp(Float) (Variables|Splat_Options|GetSplatSize_Max) 1.0 999999.0) 1e+01)))))))
  (bind _asbp_bloodstain_main (Utilities|Casting|CastToBP_Bloodstain_Main _pooledactor))
  (Transformation|SetRelativeRotation (Variables|/Game/sA_BloodSplatter_System/Blueprints/BP_Bloodstain_Main.BP_Bloodstain_Main_C|GetPlane _asbp_bloodstain_main) (Math|Rotator|MakeRotator (.roll (Variables|/Script/Engine.SceneComponent|GetRelativeRotation (Variables|/Game/sA_BloodSplatter_System/Blueprints/BP_Bloodstain_Main.BP_Bloodstain_Main_C|GetPlane _asbp_bloodstain_main))) (.pitch (Variables|/Script/Engine.SceneComponent|GetRelativeRotation (Variables|/Game/sA_BloodSplatter_System/Blueprints/BP_Bloodstain_Main.BP_Bloodstain_Main_C|GetPlane _asbp_bloodstain_main))) (Math|Random|RandomFloatinRange 0.0 5e+01)) false false)
  ;;[1 0 0.3694] Random Material Section
  (bind _returnvalue (Rendering|Material|CreateDynamicMaterialInstance (Utilities|Array|Get(acopy) _splat_materials (Math|Random|RandomIntegerinRange 0 (- (Utilities|Array|Length _splat_materials) 1))) "None" "None" :!class /Script/Engine.KismetMaterialLibrary))
  (Rendering|Material|SetVectorParameterValue _returnvalue "Color" (Variables|Default|GetColor) :!class /Script/Engine.MaterialInstanceDynamic)
  (Rendering|Material|SetMaterial (Variables|/Game/sA_BloodSplatter_System/Blueprints/BP_Bloodstain_Main.BP_Bloodstain_Main_C|GetPlane _asbp_bloodstain_main) 0 _returnvalue)
  (Variables|/Game/sA_BloodSplatter_System/Blueprints/BP_Bloodstain_Main.BP_Bloodstain_Main_C|SetLifetime _asbp_bloodstain_main (Variables|Splat_Options|GetSplat_Duration))
  (for _array_element Data
    _))

(event EventSetinUse
  (params (InUse :type Boolean) (Owner :type Actor%20Object%20Reference) (DamageInfo :type S%20Damage%20Info%20Structure))
  (|CallParentFunction InUse 0 "")
  (if InUse
    (Components|Activation|Activate (Variables|Default|GetDropletStyle_Niagara) false)
    (else
      (Components|Activation|Deactivate (Variables|Default|GetDropletStyle_Niagara)))))

(event EventBeginPlay
  (CallFunction|SpawnDrops))

(fn ConstructionScript)